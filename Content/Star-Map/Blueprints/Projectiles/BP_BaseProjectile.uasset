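; Base projectile for the Star-Map game that flies along a set direction, damages what it hits and expires after a lifetime.
; Init configures the movement speed and picks a player or enemy sprite from the owner's team, defaulting to enemy.
; Overlaps ignoring itself and its owner send a damage message, then explode.
; Explosions, also triggered by incoming damage, spawn randomized colored spheres before destroying the projectile.
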(event OnComponentBeginOverlap(collider)
  (params (OverlappedComponent :type Primitive%20Component%20Object%20Reference) (OtherActor :type Actor%20Object%20Reference) (OtherComp :type Primitive%20Component%20Object%20Reference) (OtherBodyIndex :type Integer) (bFromSweep :type Boolean) (SweepResult :type Hit%20Result%20Structure%20%28by%20ref%29))
  (bind _returnvalue (Components|GetOwner))
  (bind _returnvalue_2 (Components|GetOwner OtherComp))
  (if (!= _returnvalue_2 self)
    (if (!= _returnvalue_2 _returnvalue)
      (Class|IDamage|ApplyDamage(Message) _returnvalue_2 (Variables|bulletSettings|GetDamage) _returnvalue)
      (CallFunction|Explode))))

(event EventApplyDamage
  (params (Damage :type Float%20%28single-precision%29) (Instigator :type Actor%20Object%20Reference))
  (CallFunction|Explode))

(event EventBeginPlay
  (CallFunction|Init)
  (Utilities|FlowControl|Delay (Variables|bulletSettings|GetlifeTime))
  (Actor|DestroyActor))

(fn ConstructionScript)

(fn Init
  (bind _projectilemovement (Variables|Default|GetProjectileMovement))
  (bind _speed (Variables|bulletSettings|GetSpeed))
  (Variables|/Script/Engine.ProjectileMovementComponent|SetMaxSpeed _projectilemovement _speed)
  (bind _output_get (Variables|/Script/Engine.ProjectileMovementComponent|SetInitialSpeed _projectilemovement _speed))
  (Variables|/Script/Engine.MovementComponent|SetVelocity _projectilemovement (* (Variables|BulletSettings|Getdirection) _output_get))
  (bind (_isvalid _team) (Class|ITeams|GetTeam(Message) (Components|GetOwner)))
  (if _isvalid
    (switch Utilities|FlowControl|Switch|SwitchonE_Teams _team
      (:NewEnumerator0
        (Rendering|Components|Sprite|SetSprite (Variables|Default|GetPaperSprite) (Variables|Default|GetPlayerSprite)))
      (:NewEnumerator1
        (Rendering|Components|Sprite|SetSprite (Variables|Default|GetPaperSprite) (Variables|Default|GetEnemySprite) :!label _label)))
    (else
      (goto _label))))

(fn SpawnExplosionVFX
  (bind _output_get (LocalVariables|SetnToSPawn (Math|Random|RandomIntegerinRange (Variables|ExplosionVFX|GetnMinExplosions) (Variables|ExplosionVFX|GetnMaxExplosions))))
  (for _index (range 0 (- _output_get 1))
    (bind _returnvalue (Game|SpawnActorfromClass "/Game/Star-Map/Blueprints/VFX/ExplosionSphere.ExplosionSphere_C" (Math|Transform|MakeTransform "0, 0, 0" "0, 0, 0" "1,1,1") "Undefined" 0 0))
    (Utilities|Array|Add (LocalVariables|Getexplosions) _returnvalue))
  (for _array_element (LocalVariables|Getexplosions)
    (Default|InitSphere _array_element (Math|Random|RandomFloatinRange (Variables|ExplosionVFX|GetminSize) (Variables|ExplosionVFX|GetmaxSize)) (Math|Random|RandomFloatinRange (Variables|ExplosionVFX|GetMinDuration) (Variables|ExplosionVFX|GetmaxDuration)) (Utilities|Array|Get(acopy) (Variables|ExplosionVFX|GetexplosionColours) (Math|Random|RandomIntegerinRange 0 (Utilities|Array|LastIndex (Variables|ExplosionVFX|GetexplosionColours)))) (+ (Transformation|GetActorLocation) (Math|Vector|MakeVector (Math|Random|RandomFloatinRange (Variables|ExplosionVFX|GetminOffset) (Variables|ExplosionVFX|GetmaxOffset)) (Math|Random|RandomFloatinRange (Variables|ExplosionVFX|GetminOffset) (Variables|ExplosionVFX|GetmaxOffset)) (Math|Random|RandomFloatinRange (Variables|ExplosionVFX|GetminOffset) (Variables|ExplosionVFX|GetmaxOffset)))))))

(fn Explode
  (CallFunction|SpawnExplosionVFX)
  (Utilities|IsValid self
    (:Is%20Valid
      (Actor|DestroyActor))))