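; BP_HomingMissile is a projectile that locks onto non-team actors entering its detection collider and steers toward them.
; On overlap, it skips actors sharing its owner, checks team membership through team message calls, then stores the target and enables homing.
; Each tick, it interpolates its yaw toward the target at TurnRate and realigns velocity to its forward vector, preserving speed.
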(event OnComponentBeginOverlap(DetectionCollider)
  (params (OverlappedComponent :type Primitive%20Component%20Object%20Reference) (OtherActor :type Actor%20Object%20Reference) (OtherComp :type Primitive%20Component%20Object%20Reference) (OtherBodyIndex :type Integer) (bFromSweep :type Boolean) (SweepResult :type Hit%20Result%20Structure%20%28by%20ref%29))
  (bind _returnvalue (Components|GetOwner OtherComp))
  (if (!= (Components|GetOwner _returnvalue) (Components|GetOwner))
    (bind (_isvalid _team) (Class|ITeams|GetTeam(Message) (Components|GetOwner)))
    (if _isvalid
      (bind (_isteammember _isvalid_2) (Class|ITeams|IsonTeam(Message) _returnvalue _team))
      (if (and (not _isteammember) _isvalid_2)
        (Variables|/Script/Engine.ProjectileMovementComponent|SetbIsHomingProjectile (Variables|Default|GetProjectileMovement) true)
        (Variables|Default|Settarget _returnvalue)))))

(event EventBeginPlay
  (|CallParentFunction) ; This node is disabled and will not be called.\nDrag off pins to build functionality.
)

(event EventTick
  (params (DeltaSeconds :type Float%20%28single-precision%29))
  (if (Variables|/Script/Engine.ProjectileMovementComponent|GetbIsHomingProjectile (Variables|Default|GetProjectileMovement))
    (Utilities|IsValid (Variables|Default|Gettarget)
      (:Is%20Valid
        (Transformation|SetActorRelativeRotation (Math|Rotator|MakeRotator 0.0 0.0 (.yaw (Math|Interpolation|RInterpTo (Transformation|GetActorRotation) (Math|Rotator|FindLookatRotation (Transformation|GetActorLocation) (Transformation|GetActorLocation (Variables|Default|Gettarget))) DeltaSeconds (Variables|Default|GetTurnRate)))))
        (Variables|/Script/Engine.MovementComponent|SetVelocity (Variables|Default|GetProjectileMovement) (* (Transformation|GetActorForwardVector) (Math|Vector|VectorLength (Variables|/Script/Engine.MovementComponent|GetVelocity (Variables|Default|GetProjectileMovement)))))))))

(fn ConstructionScript
  (|CallParentFunction))