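; Base ship actor that turns toward the player's mouse cursor, moves by thrust and strafe, and fires primary guns.
; Tick interpolates yaw toward the cursor's visibility-trace hit point at the ship's turn rate.
; Input events feed forces and braking state into BPSpaceShipMovement, initialized with the ship's mass and brake rate.
; While firing is held, each tick messages every enabled weapon child actor in the four gun ports.
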(event EventOnBrake
  ;[1 1 1] On Movement Input
  (Default|SetIsBraking (Variables|Default|GetBP_SpaceShipMovement) true))

(event EventOnStopBraking
  ;[1 1 1] On Movement Input
  (Default|SetIsBraking (Variables|Default|GetBP_SpaceShipMovement) false))

(event EventTick
  (params (DeltaSeconds :type Float%20%28single-precision%29))
  (Transformation|SetActorRelativeRotation (Math|Rotator|MakeRotator 0.0 0.0 (.yaw (Math|Interpolation|RInterpTo (Transformation|GetActorRotation) (Math|Rotator|FindLookatRotation (Transformation|GetActorLocation) (.impactpoint (.HitResult (Game|Player|GetHitResultUnderCursorbyChannel (Game|GetPlayerController 0) "TraceTypeQuery1" true)))) DeltaSeconds (Variables|FlySettings|GetTurnRate)))))
  (if (Variables|ShipStates|GetIsPrimaryFiring)
    (CallFunction|FirePrimaryGuns)))

(event EventOnFirePrimary
  ;[1 1 1] Firing Weapons
  (Variables|ShipStates|SetIsPrimaryFiring true))

(event EventOnStopFiringPrimary
  ;[1 1 1] Firing Weapons
  (Variables|ShipStates|SetIsPrimaryFiring false))

(event EventApplyStrafe
  (params (Axis :type Float%20%28single-precision%29))
  ;[1 1 1] On Movement Input
  (Default|ApplyForce (Variables|Default|GetBP_SpaceShipMovement) (* (* (Transformation|GetActorRightVector) Axis) (Variables|FlySettings|GetStrafeForce))))

(event EventApplyThrust
  (params (Axis :type Float%20%28single-precision%29))
  ;[1 1 1] On Movement Input
  (Default|ApplyForce (Variables|Default|GetBP_SpaceShipMovement) (* (* (Transformation|GetActorForwardVector) Axis) (Variables|FlySettings|GetThrustForce))))

(event EventBeginPlay
  (CallFunction|Init)
  (Default|Init (Variables|Default|GetBP_SpaceShipMovement) (Variables|ShipSettings|GetShip%20Mass) (Variables|FlySettings|GetBrake%20Rate) 5e+03))

(fn ConstructionScript)

(fn Init
  (Utilities|Array|Add (Variables|ShipModules|GetGunPorts) (Variables|Default|GetWeaponPort))
  (Utilities|Array|Add (Variables|ShipModules|GetGunPorts) (Variables|Default|GetWeaponPort1))
  (Utilities|Array|Add (Variables|ShipModules|GetGunPorts) (Variables|Default|GetWeaponPort3))
  (Utilities|Array|Add (Variables|ShipModules|GetGunPorts) (Variables|Default|GetWeaponPort4)))

(fn FirePrimaryGuns
  (for _array_element (Variables|ShipModules|GetGunPorts)
    (bind _isenabled (Class|IShipWeapon|IsEnabled(Message) (Variables|/Script/Engine.ChildActorComponent|GetChildActor _array_element)))
    (if _isenabled
      (Class|IShipWeapon|UseWeapon(Message) (Variables|/Script/Engine.ChildActorComponent|GetChildActor _array_element) self))))