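; BP_Turret is a destructible, team-assigned turret that tracks and fires on the player.
; Its detection sphere sets or clears the target as actors tagged Player enter and leave.
; Each tick it smoothly interpolates its yaw toward the target and, within range, messages its child-actor weapon to fire, without checking aim.
; ApplyDamage reduces health and destroys the turret at zero, while team queries do not affect targeting.
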(event OnComponentBeginOverlap(DetectionSphere)
  (params (OverlappedComponent :type Primitive%20Component%20Object%20Reference) (OtherActor :type Actor%20Object%20Reference) (OtherComp :type Primitive%20Component%20Object%20Reference) (OtherBodyIndex :type Integer) (bFromSweep :type Boolean) (SweepResult :type Hit%20Result%20Structure%20%28by%20ref%29))
  (if (Actor|ActorHasTag (Components|GetOwner OtherComp) "Player")
    (Variables|Settings|SetCanLockOn true)
    (Variables|Settings|SetTarget OtherActor)))

(event OnComponentEndOverlap(DetectionSphere)
  (params (OverlappedComponent :type Primitive%20Component%20Object%20Reference) (OtherActor :type Actor%20Object%20Reference) (OtherComp :type Primitive%20Component%20Object%20Reference) (OtherBodyIndex :type Integer))
  (if (Actor|ActorHasTag (Components|GetOwner OtherComp) "Player")
    (Variables|Settings|SetCanLockOn false)
    (Variables|Settings|SetTarget 0)))

(event EventBeginPlay
  (Variables|Default|SetCurrentHealth (Variables|Default|GetMaxHealth)))

(event EventApplyDamage
  (params (Damage :type Float%20%28single-precision%29) (Instigator :type Actor%20Object%20Reference))
  (bind _output_get (Variables|Default|SetCurrentHealth (- (Variables|Default|GetCurrentHealth) Damage)))
  (if (<= _output_get 0.0)
    (Actor|DestroyActor)))

(event EventTick
  (params (DeltaSeconds :type Float%20%28single-precision%29))
  (if (Variables|Settings|GetCanLockOn)
    (Utilities|IsValid (Variables|Settings|GetTarget)
      (:Is%20Valid
        (Transformation|SetActorRelativeRotation (Math|Rotator|MakeRotator 0.0 0.0 (.yaw (Math|Interpolation|RInterpTo (Transformation|GetActorRotation) (Math|Rotator|FindLookatRotation (Transformation|GetActorLocation) (Transformation|GetActorLocation (Variables|Settings|GetTarget))) DeltaSeconds (Variables|Settings|GetrotationRate)))))
        (if (<= (Math|Vector|VectorLength (- (Transformation|GetActorLocation (Variables|Settings|GetTarget)) (Transformation|GetActorLocation))) (Variables|Settings|Getrange))
          (Class|IShipWeapon|UseWeapon(Message) (Variables|/Script/Engine.ChildActorComponent|GetChildActor (Variables|Default|GetChildActor)) self))))))

(fn ConstructionScript)

(fn GetTeam
  (return true (Variables|Default|GetTeam)))

(fn IsonTeam
  (params (OtherTeam :type E_Teams%20Enum :default "NewEnumerator0"))
  (return (Utilities|Enum|Equal(Enum) OtherTeam (Variables|Default|GetTeam)) true))