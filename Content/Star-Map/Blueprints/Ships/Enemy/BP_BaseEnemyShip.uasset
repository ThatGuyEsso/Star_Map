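; Base Blueprint for AI enemy ships in the star map, with team-based target detection.
; Init spawns its AI controller, loads AI data from a DataTable row to size the detection sphere, and initializes shield/health, movement and steering components.
; Sphere overlaps set Target to the overlapping owner when it is validly on another team.
; A helper smoothly yaws the ship toward its velocity at its turn rate.
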(event OnComponentBeginOverlap(Detection)
  (params (OverlappedComponent :type Primitive%20Component%20Object%20Reference) (OtherActor :type Actor%20Object%20Reference) (OtherComp :type Primitive%20Component%20Object%20Reference) (OtherBodyIndex :type Integer) (bFromSweep :type Boolean) (SweepResult :type Hit%20Result%20Structure%20%28by%20ref%29))
  (bind _returnvalue (Components|GetOwner OtherActor))
  (if (!= _returnvalue self)
    (bind (_isteammember _isvalid) (Class|ITeams|IsonTeam(Message) _returnvalue (Variables|Default|GetTeam)))
    (if (and (not _isteammember) _isvalid)
      (Variables|AISettings|SetTarget _returnvalue))))

(event EventTick
  (params (DeltaSeconds :type Float%20%28single-precision%29)))

(fn ConstructionScript
  (|CallParentFunction))

(fn Init
  (|CallParentFunction)
  (CallFunction|CreateController)
  (CallFunction|SetAIData (Variables|Default|GetAI_DT) (Variables|Default|GetDT_AI_Name))
  (Default|Init (Variables|Default|GetBPC_Shield_And_Health) (Variables|Default|GetMaxShieldHealth) (Variables|Default|GetMaxHullHealth) (Variables|Default|GetShieldRechargeRate) (Variables|Default|GetShortShieldRechargeCoolDown) (Variables|Default|GetLongShieldRechargeCoolDown))
  (Default|Init (Variables|Default|GetBP_SpaceShipMovement) (Variables|Default|GetShip%20Mass) (Variables|Default|GetBrake%20Rate) (.maxspeed (Variables|Default|GetShipData)))
  (Default|Init (Variables|Default|GetBPC_SteeringManager) (Variables|Default|GetBP_SpaceShipMovement)))

(fn CreateController
  (bind _returnvalue (Game|SpawnActorfromClass "/Game/Star-Map/Blueprints/Controllers/AIC_BaseEnemyShip.AIC_BaseEnemyShip_C" (Math|Transform|MakeTransform "0, 0, 0" "0, 0, 0" "1,1,1") "Undefined" 0 0))
  (bind _output_get (Variables|Default|SetAIContronller _returnvalue))
  (Class|IAIController|Init(Message) _output_get self))

(fn SetAIData
  (params (DataTable :type Data%20Table%20Object%20Reference) (RowName :type Name))
  (bind _returnvalue (Utilities|GetDataTableRow DataTable RowName)
    (:then
      (bind _output_get (Variables|AISettings|SetAIData _returnvalue))
      (bind _structout (Utilities|Struct|SetmembersinS_AIData _output_get))
      (Components|Sphere|SetSphereRadius (Variables|Default|GetDetection) (.DetectionRange (Utilities|Struct|BreakS_AIData _structout)) true))))

(fn FaceMovementDirection
  (params (DeltaTime :type Float%20%28single-precision%29))
  (if (> (Math|Vector|VectorLength (Transformation|GetVelocity)) 0.0)
    (Transformation|SetActorRelativeRotation (Math|Rotator|MakeRotator 0.0 0.0 (.yaw (Math|Interpolation|RInterpTo (Transformation|GetActorRotation) (Math|Rotator|FindLookatRotation (Transformation|GetActorLocation) (Transformation|GetVelocity)) DeltaTime (.turnrate (Variables|Default|GetShipData))))))))

(fn GetAIData
  (return (Variables|AISettings|GetAIData)))