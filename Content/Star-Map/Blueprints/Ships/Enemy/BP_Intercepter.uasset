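; BP_Intercepter is an enemy interceptor ship that moves using steering behaviors.
; Init configures its steering manager with speed, acceleration, deceleration and recovery limits.
; OnSeek gets a force toward a target point from the seek component and adds it to the manager.
; Each tick the ship faces its movement direction and updates steering, and it exposes BodyCollider as its main collider.
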(event EventBeginPlay
  (|CallParentFunction)
  (CallFunction|Init))

(event Collision|EventActorBeginOverlap
  (params (OtherActor :type Actor%20Object%20Reference))
  (|CallParentFunction OtherActor) ; This node is disabled and will not be called.\nDrag off pins to build functionality.
)

(event EventTick
  (params (DeltaSeconds :type Float%20%28single-precision%29))
  (|CallParentFunction DeltaSeconds)
  (CallFunction|FaceMovementDirection DeltaSeconds)
  (Default|UpdateSteering (Variables|Default|GetBPC_SteeringManager)))

(event EventOnSeek
  (params (point :type Vector :default "0, 0, 0"))
  (bind _desired_force (Default|Seek (Variables|Default|GetBPC_Seek) (Transformation|GetActorLocation) point 0.0))
  (Default|AddSteeringForce (Variables|Default|GetBPC_SteeringManager) _desired_force))

(fn ConstructionScript
  (|CallParentFunction))

(fn Init
  (|CallParentFunction)
  (Default|Init (Variables|Default|GetBPC_SteeringManager) (Utilities|Struct|MakeS_ShipMovementData 1e+04 5e+03 3e+03 9e+03)))

(fn GetMainCollider
  (return (Variables|Default|GetBodyCollider)))