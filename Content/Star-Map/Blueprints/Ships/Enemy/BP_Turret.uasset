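; Enemy turret that locks onto players entering its detection sphere, turns smoothly in yaw toward them and fires within range.
; Init picks a random weapon from the current level's data table row and sets it as its weapon port's child actor, optionally spawning a platform beneath.
; Weapons are driven by messages each tick, with lasers also toggled on overlap.
; At zero health it spawns an explosion and destroys itself.
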(event OnComponentBeginOverlap(DetectionSphere)
  (params (OverlappedComponent :type Primitive%20Component%20Object%20Reference) (OtherActor :type Actor%20Object%20Reference) (OtherComp :type Primitive%20Component%20Object%20Reference) (OtherBodyIndex :type Integer) (bFromSweep :type Boolean) (SweepResult :type Hit%20Result%20Structure%20%28by%20ref%29))
  (bind _returnvalue (Components|GetOwner OtherComp))
  (if (Actor|ActorHasTag _returnvalue "Player")
    (Variables|Settings|SetCanLockOn true)
    (Variables|Settings|SetTarget _returnvalue)
    (switch Utilities|FlowControl|Switch|SwitchonE_WeaponType (Variables|TurretSettings|GetTurretType)
      (:NewEnumerator3
        (CallFunction|UseWeapons)))))

(event OnComponentEndOverlap(DetectionSphere)
  (params (OverlappedComponent :type Primitive%20Component%20Object%20Reference) (OtherActor :type Actor%20Object%20Reference) (OtherComp :type Primitive%20Component%20Object%20Reference) (OtherBodyIndex :type Integer))
  (if (Actor|ActorHasTag (Components|GetOwner OtherComp) "Player")
    (Variables|Settings|SetCanLockOn false)
    (Variables|Settings|SetTarget 0)
    (switch Utilities|FlowControl|Switch|SwitchonE_WeaponType (Variables|TurretSettings|GetTurretType)
      (:NewEnumerator3
        (CallFunction|StopUsingWeapons)))))

(event EventBeginPlay
  (Utilities|FlowControl|Delay 0.5)
  (CallFunction|Init))

(event EventApplyDamage
  (params (Damage :type Float%20%28single-precision%29) (Instigator :type Actor%20Object%20Reference))
  (bind _output_get (Variables|TurretSettings|SetCurrentHealth (- (Variables|TurretSettings|GetCurrentHealth) Damage)))
  (if (<= _output_get 0.0)
    (Game|SpawnActorfromClass :Class "/Game/Star-Map/Blueprints/VFX/BP_ExplosionManager.BP_ExplosionManager_C" :SpawnTransform (Math|Transform|MakeTransform (Transformation|GetActorLocation) "0, 0, 0" "1,1,1") :CollisionHandlingOverride "Undefined" :Settings (Variables|Default|GetExplosionSettings) :Instigator 0)
    (Actor|DestroyActor)))

(event EventTick
  (params (DeltaSeconds :type Float%20%28single-precision%29))
  (if (Variables|Settings|GetCanLockOn)
    (Utilities|IsValid (Variables|Settings|GetTarget)
      (:Is%20Valid
        (Transformation|SetActorRelativeRotation (Math|Rotator|MakeRotator 0.0 0.0 (.yaw (Math|Interpolation|RInterpTo (Transformation|GetActorRotation) (Math|Rotator|FindLookatRotation (Transformation|GetActorLocation) (Transformation|GetActorLocation (Variables|Settings|GetTarget))) DeltaSeconds (Variables|Settings|GetrotationRate)))))
        (if (<= (Math|Vector|VectorLength (- (Transformation|GetActorLocation (Variables|Settings|GetTarget)) (Transformation|GetActorLocation))) (Variables|Settings|Getrange))
          (for _array_element (Variables|TurretSettings|GetWeaponPorts)
            (Class|IShipWeapon|UseWeapon(Message) (Variables|/Script/Engine.ChildActorComponent|GetChildActor _array_element) self)))))))

(fn ConstructionScript)

(fn GetAvailableWeapons
  (params (DataTable :type Data%20Table%20Object%20Reference) (RowName :type Name))
  (bind _returnvalue (Utilities|GetDataTableRow DataTable RowName)
    (:then
      (Variables|TurretData|SetAvailableWeapons _returnvalue))))

(fn Init
  (CallFunction|GetAllWeaponPorts)
  (Variables|TurretSettings|SetCurrentHealth (Variables|TurretSettings|GetMaxHealth))
  (bind _levelname (Class|IGameMode|GetCurrentLevelName(Message) (Game|GetGameMode)))
  (CallFunction|GetAvailableWeapons (Variables|TurretData|GetAvailableWeaponsDT) (Utilities|String|StringToName _levelname))
  (CallFunction|AddWeapons)
  (if (Variables|Default|GetShouldSpawnPlatform)
    (CallFunction|SpawnPlatform))
  (Default|OnInit (Variables|Default|GetBPC_PointsOfInterest)))

(fn GetAllWeaponPorts
  (Utilities|Array|Add (Variables|TurretSettings|GetWeaponPorts) (Variables|Default|GetWeaponPort)))

(fn AddWeapons
  (bind _self self)
  (bind _availableweapons (Variables|TurretData|GetAvailableWeapons))
  (bind _weapon (Utilities|Struct|BreakS_AvailableEnemyWeapons _availableweapons))
  (bind _output_get (LocalVariables|SetIndex (Math|Random|RandomIntegerinRange 0 (Utilities|Array|LastIndex _weapon))))
  (LocalVariables|SetWeaponSetting (Utilities|Array|Get(acopy) _weapon _output_get))
  (for _array_element (Variables|TurretSettings|GetWeaponPorts)
    (LocalVariables|SetCurrentWeaponPort _array_element)
    (Variables|TurretSettings|SetTurretType (.weapontype (LocalVariables|GetWeaponSetting)))
    (switch Utilities|FlowControl|Switch|SwitchonE_WeaponType (.weapontype (LocalVariables|GetWeaponSetting))
      (:NewEnumerator0
        (ChildActorComponent|SetChildActorClass (LocalVariables|GetCurrentWeaponPort) "/Game/Star-Map/Blueprints/Weapons/BP_BaseGun.BP_BaseGun_C")
        (Class|IShipWeapon|InitWeapon(Message) (Variables|/Script/Engine.ChildActorComponent|GetChildActor (LocalVariables|GetCurrentWeaponPort)) "NewEnumerator1" _self))
      (:NewEnumerator1
        (ChildActorComponent|SetChildActorClass (LocalVariables|GetCurrentWeaponPort) "/Game/Star-Map/Blueprints/Weapons/BP_MissileLauncher.BP_MissileLauncher_C")
        (Class|IShipWeapon|InitWeapon(Message) (Variables|/Script/Engine.ChildActorComponent|GetChildActor (LocalVariables|GetCurrentWeaponPort)) "NewEnumerator1" _self))
      (:NewEnumerator2
        (ChildActorComponent|SetChildActorClass (LocalVariables|GetCurrentWeaponPort) "/Game/Star-Map/Blueprints/Weapons/BP_HomingMissileLauncher.BP_HomingMissileLauncher_C")
        (Class|IShipWeapon|InitWeapon(Message) (Variables|/Script/Engine.ChildActorComponent|GetChildActor (LocalVariables|GetCurrentWeaponPort)) "NewEnumerator1" _self))
      (:NewEnumerator3
        (ChildActorComponent|SetChildActorClass (LocalVariables|GetCurrentWeaponPort) "/Game/Star-Map/Blueprints/Weapons/BP_H_I_Laser.BP_H_I_Laser_C")
        (Class|IShipWeapon|InitWeapon(Message) (Variables|/Script/Engine.ChildActorComponent|GetChildActor (LocalVariables|GetCurrentWeaponPort)) "NewEnumerator1" _self)))
    (Class|IShipWeapon|SetWeaponSettings(Message) (Variables|/Script/Engine.ChildActorComponent|GetChildActor (LocalVariables|GetCurrentWeaponPort)) (LocalVariables|GetWeaponSetting))
    (Class|IShipWeapon|InitWeapon(Message) (Variables|/Script/Engine.ChildActorComponent|GetChildActor (LocalVariables|GetCurrentWeaponPort)) "NewEnumerator1" self)))

(fn UseWeapons
  (for _array_element (Variables|TurretSettings|GetWeaponPorts)
    (Class|IShipWeapon|SetIsAttacking(Message) (Variables|/Script/Engine.ChildActorComponent|GetChildActor _array_element) true)))

(fn StopUsingWeapons
  (for _array_element (Variables|TurretSettings|GetWeaponPorts)
    (Class|IShipWeapon|SetIsAttacking(Message) (Variables|/Script/Engine.ChildActorComponent|GetChildActor _array_element) false)))

(fn SpawnPlatform
  (bind _returnvalue (Transformation|GetActorLocation))
  (Game|SpawnActorfromClass "/Game/Star-Map/Blueprints/SceneActors/BP_Platform.BP_Platform_C" (Math|Transform|MakeTransform (Math|Vector|MakeVector (.x _returnvalue) (.y _returnvalue) (- (.z _returnvalue) 2.5e+02)) "0, 0, 0" "1,1,1") "Undefined" 0 self 0))

(fn GetMeshComponent
  (return (Variables|Default|GetMesh)))

(fn GetTeam
  (return true "NewEnumerator1"))

(fn IsonTeam
  (params (OtherTeam :type E_Teams%20Enum :default "NewEnumerator0"))
  (return (Utilities|Enum|Equal(Enum) OtherTeam "NewEnumerator1") true))