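; BP_DualTurret is an enemy ship turret Blueprint with two weapon ports.
; Its GetAllWeaponPorts function adds WeaponPort and WeaponPort1 to the WeaponPorts array.
; The event graph holds only disabled default nodes, and the construction script just calls its parent.
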(event EventBeginPlay
  (|CallParentFunction) ; This node is disabled and will not be called.\nDrag off pins to build functionality.
)

(event Collision|EventActorBeginOverlap
  (params (OtherActor :type Actor%20Object%20Reference)))

(event EventTick
  (params (DeltaSeconds :type Float%20%28single-precision%29))
  (|CallParentFunction DeltaSeconds) ; This node is disabled and will not be called.\nDrag off pins to build functionality.
)

(fn ConstructionScript
  (|CallParentFunction))

(fn GetAllWeaponPorts
  (bind _weaponports (Variables|Default|GetWeaponPorts))
  (Utilities|Array|Add _weaponports (Variables|Default|GetWeaponPort))
  (Utilities|Array|Add _weaponports (Variables|Default|GetWeaponPort1)))