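; Player-controlled ship that turns to face the mouse cursor, takes thrust, strafe and brake input, and fires primary guns while held.
; Movement and shield/hull components handle flight and damage, with health changes pushed to the player HUD.
; Child-actor gun ports host weapons that toggle by type and report to the HUD.
; A spawned raycast floor, initialised with the ship as target and an offset below it, accompanies the cursor-trace aiming.
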(event Custom|OnHealthUpdate
  (params (newHealth :type Float%20%28single-precision%29))
  (CallFunction|UpdateHealthDisplay))

(event Custom|OnShieldUpdate
  (params (NewShieldHealth :type Float%20%28single-precision%29))
  (CallFunction|UpdateShieldDisplay))

(event EventOnBrake
  ;[1 1 1] On Movement Input
  (Variables|/Game/Star-Map/Blueprints/Components/BPC_ShipMovement.BPC_ShipMovement_C|SetIsBraking (Variables|Default|GetBPC_ShipMovement) true))

(event EventOnStopBraking
  ;[1 1 1] On Movement Input
  (Variables|/Game/Star-Map/Blueprints/Components/BPC_ShipMovement.BPC_ShipMovement_C|SetIsBraking (Variables|Default|GetBPC_ShipMovement) false))

(event EventOnDisplayWeapons
  (CallFunction|DiplayEquippedWeapons))

(event EventOnStopThrusting
  ;[1 1 1] On Movement Input
  (Variables|/Game/Star-Map/Blueprints/Components/BPC_ShipMovement.BPC_ShipMovement_C|SetIsTryingToAccelerate (Variables|Default|GetBPC_ShipMovement) false))

(event EventTick
  (params (DeltaSeconds :type Float%20%28single-precision%29))
  (Transformation|SetActorRelativeRotation (Math|Rotator|MakeRotator 0.0 0.0 (.yaw (Math|Interpolation|RInterpTo (Transformation|GetActorRotation) (Math|Rotator|FindLookatRotation (Transformation|GetActorLocation) (.impactpoint (.HitResult (Game|Player|GetHitResultUnderCursorbyChannel (Game|GetPlayerController 0) "TraceTypeQuery3" true)))) DeltaSeconds (.turnrate (Variables|Default|GetShipData))))))
  (if (Variables|Default|GetIsPrimaryFiring)
    (CallFunction|FirePrimaryGuns)))

(event EventOnFirePrimary
  ;[1 1 1] Firing Weapons
  (Variables|Default|SetIsPrimaryFiring true)
  (Default|CallOnTryingtoAttack))

(event EventOnStopFiringPrimary
  ;[1 1 1] Firing Weapons
  (Variables|Default|SetIsPrimaryFiring false)
  (Default|CallOnStopTryingtoAttack))

(event EventApplyStrafe
  (params (Axis :type Float%20%28single-precision%29))
  ;[1 1 1] On Movement Input
  (Variables|Default|SetInputDir (Math|Vector|MakeVector (.x (Variables|Default|GetInputDir)) Axis 0.0)))

(event EventOnApplyThrust
  ;[1 1 1] On Movement Input
  (Variables|/Game/Star-Map/Blueprints/Components/BPC_ShipMovement.BPC_ShipMovement_C|SetIsTryingToAccelerate (Variables|Default|GetBPC_ShipMovement) true))

(event EventBeginPlay
  (CallFunction|Init)
  (Default|Init (Variables|Default|GetBPC_ShipMovement) (Utilities|Struct|MakeS_ShipMovementData 1e+04 5e+03 3e+03 9e+03))
  (EventDispatchers|BindEventtoOnHullHealthUpdated (Variables|Default|GetBPC_Shield_And_Health) (delegate Custom|OnHealthUpdate))
  (EventDispatchers|BindEventtoOnShieldHealthUpdated (Variables|Default|GetBPC_Shield_And_Health) (delegate Custom|OnShieldUpdate))
  (Utilities|FlowControl|Delay 0.2)
  (CallFunction|UpdateShieldDisplay)
  (CallFunction|UpdateHealthDisplay))

(event EventApplyDamage
  (params (Damage :type Float%20%28single-precision%29) (Instigator :type Actor%20Object%20Reference))
  (Default|OnDamageTaken (Variables|Default|GetBPC_Shield_And_Health) Damage))

(event EventOnToggleWeaponsOfType
  (params (type :type E_WeaponType%20Enum :default "NewEnumerator0"))
  (CallFunction|ToggleWeaponsOfType type))

(fn ConstructionScript
  (|CallParentFunction))

(fn UpdateShieldDisplay
  (bind _hud (Class|IPlayerController|GetPlayerHUD(Message) (Game|GetPlayerController 0)))
  (bind (_current _max) (Default|GetShieldData (Variables|Default|GetBPC_Shield_And_Health)))
  (Default|UpdateShield _hud (/ _current _max)))

(fn UpdateHealthDisplay
  (bind _hud (Class|IPlayerController|GetPlayerHUD(Message) (Game|GetPlayerController 0)))
  (bind (_current _max) (Default|GetHullData (Variables|Default|GetBPC_Shield_And_Health)))
  (Default|UpdateHealth _hud (/ _current _max)))

(fn RegisterPorts
  (Utilities|Array|Add (Variables|Default|GetGunPorts) (Variables|Default|GetWeaponPort))
  (Utilities|Array|Add (Variables|Default|GetGunPorts) (Variables|Default|GetWeaponPort2))
  (Utilities|Array|Add (Variables|Default|GetGunPorts) (Variables|Default|GetWeaponPort3))
  (for _array_element (Variables|Default|GetGunPorts)
    (Class|IShipWeapon|InitWeapon(Message) (Variables|/Script/Engine.ChildActorComponent|GetChildActor _array_element) "NewEnumerator0" self)))

(fn Init
  (bind _shipdata (Variables|Default|GetShipData))
  (|CallParentFunction)
  (Default|Init (Variables|Default|GetBPC_Shield_And_Health) (.maxshieldhealth _shipdata) (.maxhullhealth _shipdata) (.shieldrechargerate _shipdata) (.shortshieldcooldown _shipdata) (.longshieldcooldown _shipdata) (Variables|Default|GetShield%20Scale))
  (bind _returnvalue (Game|SpawnActorfromClass "/Game/Star-Map/Blueprints/Misc/BP_RaycastFloor.BP_RaycastFloor_C" (Math|Transform|MakeTransform "0, 0, 0" "0, 0, 0" "1,1,1") "Undefined" 0 0))
  (Default|Init _returnvalue self "0, 0,-200.000000"))

(fn ToggleWeaponsOfType
  (params (WeaponTyoe :type E_WeaponType%20Enum :default "NewEnumerator0"))
  (for _array_element (Variables|Default|GetGunPorts)
    (bind _type (Class|IShipWeapon|GetWeaponType(Message) (Variables|/Script/Engine.ChildActorComponent|GetChildActor _array_element)))
    (if (Utilities|Enum|Equal(Enum) _type WeaponTyoe)
      (bind _isenabled (Class|IShipWeapon|IsEnabled(Message) (Variables|/Script/Engine.ChildActorComponent|GetChildActor _array_element)))
      (Class|IShipWeapon|SetIsEnabled(Message) (Variables|/Script/Engine.ChildActorComponent|GetChildActor _array_element) (not _isenabled)))))

(fn DiplayEquippedWeapons
  (for _array_element (Variables|Default|GetGunPorts)
    (bind _hud (Class|IPlayerController|GetPlayerHUD(Message) (Pawn|GetController)))
    (bind _type (Class|IShipWeapon|GetWeaponType(Message) (Variables|/Script/Engine.ChildActorComponent|GetChildActor _array_element)))
    (bind _isenabled (Class|IShipWeapon|IsEnabled(Message) (Variables|/Script/Engine.ChildActorComponent|GetChildActor _array_element)))
    (Class|IHUD|OnAddUpdateEquippedWeapons(Message) _hud _type _isenabled)
    (Class|IShipWeapon|UpdateHUDDisplay(Message) (Variables|/Script/Engine.ChildActorComponent|GetChildActor _array_element))))

(fn GetTeam
  (return true "NewEnumerator0"))

(fn IsTryingtoAttack
  (return (Variables|Default|GetIsPrimaryFiring)))

(fn GetCurrentPercentageHealth
  (bind (_current _max) (Default|GetHullData (Variables|Default|GetBPC_Shield_And_Health)))
  (return (/ _current _max)))

(fn GetCurrentPercentageShieldHealth
  (bind (_current _max) (Default|GetShieldData (Variables|Default|GetBPC_Shield_And_Health)))
  (return (/ _current _max)))