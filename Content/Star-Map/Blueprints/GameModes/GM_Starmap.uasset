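; GM_Starmap is the level game mode for a top-down spaceship game, running play from startup to level clear or game over.
; An OnNewGameState dispatcher drives a state machine where setup steps chain into the next: actor init, player login, ship spawn, asteroid generation (awaited by event), cameras and HUD.
; It also manages loading, pause, level-select and game-over screens, loads scenes, and saves level progress through the game instance.
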(event Custom|DisplayGameOver
  ;[1 1 1] Start Game Over Sequence
  (bind _asbp_player_ship (Utilities|Casting|CastToBP_PlayerShip (Variables|PlayerComponents|GetPlayerShip)))
  (Default|DestroyShip _asbp_player_ship)
  (Utilities|FlowControl|Delay 1.0)
  (CallFunction|AddGameOverScreen))

(event Custom|OnBindToAsteroidGen
  (params (Generator :type BP%20Asteroid%20Generator%20Object%20Reference))
  ;[1 1 1] Bind and wait for Asteroid Generation To Complete
  (EventDispatchers|BindEventtoOnAsteroidGenComplete Generator (delegate Custom|OnAsteroidGenComplete)))

(event Custom|OnAsteroidGenComplete
  (bind _asteroidgenerator (Variables|SceneACtor|GetAsteroidGenerator))
  ;[1 1 1] Bind and wait for Asteroid Generation To Complete
  (Utilities|IsValid _asteroidgenerator
    (:Is%20Valid
      (EventDispatchers|UnbindEventfromOnAsteroidGenComplete _asteroidgenerator (delegate Custom|OnAsteroidGenComplete)))
    (:Is%20Not%20Valid
      _))
  (Default|CallOnNewGameState "NewEnumerator5"))

(event Custom|OnNewState
  (params (New%20GameState :type E_GameStates%20Enum :default "NewEnumerator0"))
  (bind _playershipcam (Variables|PlayerComponents|GetPlayerShipCam))
  ;[1 1 1] New Game State Events
  (bind _output_get (Variables|GameState|SetCurrentGameState New%20GameState))
  (switch Utilities|FlowControl|Switch|SwitchonE_GameStates _output_get
    (:NewEnumerator0
      (CallFunction|Init))
    (:NewEnumerator1
      (CallFunction|CreateNewController)
      (Utilities|FlowControl|Delay 0.2)
      (CallFunction|SpawnPlayerShip))
    (:NewEnumerator3
      (CallFunction|BeginAsteroidGen))
    (:NewEnumerator5
      (CallFunction|SetUpPlayerCamera))
    (:NewEnumerator6
      (CallFunction|SetUpMinimapCamera))
    (:NewEnumerator7
      (CallFunction|SetUpHUD))
    (:NewEnumerator9
      (CallFunction|StarGame))
    (:NewEnumerator12
      (CallFunction|RemovePauseScreen)
      (CallFunction|AddLevelSelectScreen))
    (:NewEnumerator13
      ;[1 1 1] Start Game Over Sequence
      (EventDispatchers|BindEventtoOnZoomComplete _playershipcam (delegate Custom|DisplayGameOver))
      (Variables|/Game/Star-Map/Blueprints/UX/BP_TopDownCamera.BP_TopDownCamera_C|SetIsFollowing _playershipcam false)
      (Default|OnZoom _playershipcam 2e+03 0.5))))

(event EventBeginPlay
  ;[1 1 1] New Game State Events
  (Utilities|FlowControl|Delay 0.2)
  (CallFunction|AddLoadingScreen)
  (EventDispatchers|BindEventtoOnNewGameState (delegate Custom|OnNewState))
  (Default|CallOnNewGameState "NewEnumerator0"))

(event EventOnTogglePause
  ;[1 1 1] On On Pause events
  (CallFunction|TogglePause))

(event EventOnGameOver
  (Default|CallOnNewGameState "NewEnumerator13"))

(event EventOnReloadLevel
  (bind _returnvalue (Game|GetCurrentLevelName true))
  (Game|OpenLevel(byName) (Utilities|String|StringToName _returnvalue)))

(event EventPostLogin
  (params (NewPlayer :type Player%20Controller%20Object%20Reference))
  ;[1 1 1] On Login
  (bind _aspc_player_ship_controller (Utilities|Casting|CastToPC_PlayerShipController NewPlayer))
  (if (Utilities|Enum|Equal(Enum) (Variables|GameState|GetCurrentGameState) "NewEnumerator1")
    (Variables|PlayerComponents|SetP%20Controller _aspc_player_ship_controller)))

(event EventDisplayLoading
  ;[1 1 1] On Begin Loading events
  (CallFunction|AddLoadingScreen))

(event EventHideLoading
  ;[1 1 1] On Begin Loading events
  (CallFunction|RemoveLoadingScreen))

(event EventLoadScene
  (params (Scene :type E_Scenes%20Enum :default "NewEnumerator2"))
  ;[1 1 1] On Load New Scene
  (Class|IGameInstance|OnSaveGame(Message) (Game|GetGameInstance))
  (bind _scenename (CallFunction|EvaluateScene Scene))
  (Game|OpenLevel(byName) (Utilities|String|StringToName _scenename)))

(event EventOnUnpause
  ;[1 1 1] On On Pause events
  (CallFunction|SetIsGamePaused false)
  (CallFunction|RemovePauseScreen))

(event EventOnPause
  ;[1 1 1] On On Pause events
  (CallFunction|SetIsGamePaused true)
  (CallFunction|AddPauseScreeen))

(event EventOnLevelClear
  (bind _returnvalue (Game|GetGameInstance))
  (bind _returnvalue_2 (Game|GetGameInstance))
  ;[1 1 1] If current level number is greater than number of completed level. It's the first time player played this level hence increase n levels complete
  (CallFunction|AddLoadingScreen)
  (bind _number (Class|IGameInstance|GetCurrentLevelNumber(Message) _returnvalue))
  (bind _data (Class|IGameInstance|GetGameData(Message) _returnvalue))
  (if (> _number (.levelscomplete _data))
    ;[1 1 1] Save Current Data
    (bind _result (Math|Integer|IncrementInt (.levelscomplete _data))
      (:%20%20
        (Class|IGameInstance|SetGameData(Message) _returnvalue_2 (Utilities|Struct|MakeS_StarmapGameData (.credits _data) _result (.playershiploadout _data) 0))))
    (else
      (Class|IGameInstance|SetGameData(Message) _returnvalue_2 (Utilities|Struct|MakeS_StarmapGameData (.credits _data) (.levelscomplete _data) (.playershiploadout _data) 0))))
  (Class|IGameInstance|OnSaveGame(Message) (Game|GetGameInstance))
  (Default|CallOnNewGameState "NewEnumerator12"))

(event EventSetCanEndGame
  (params (CanEndGame :type Boolean))
  (Variables|GameState|SetCan%20End%20Game CanEndGame))

(fn ConstructionScript)

(fn CreateNewController
  (Class|GameplayStatics|RemovePlayer (Game|GetPlayerController 0) true)
  (Class|GameplayStatics|CreatePlayer -1))

(fn SetUpPlayerCamera
  (bind _p_controller (Variables|PlayerComponents|GetP%20Controller))
  (Utilities|IsValid (Variables|PlayerComponents|GetPlayerShip)
    (:Is%20Valid
      (bind _returnvalue (Game|SpawnActorfromClass "/Game/Star-Map/Blueprints/UX/BP_TopDownCamera.BP_TopDownCamera_C" (Math|Transform|MakeTransform "0, 0, 0" "0, 0, 0" "1,1,1") "Undefined" 0 "0.000000,0.000000,6000.000000" (Variables|PlayerComponents|GetPlayerShip) 6e+01 2e+03 2e+01 0))
      (bind _output_get (Variables|PlayerComponents|SetPlayerShipCam _returnvalue))
      (Default|Init _output_get)
      (Utilities|IsValid _p_controller
        (:Is%20Valid
          (Game|Player|SetViewTargetwithBlend _p_controller (Variables|PlayerComponents|GetPlayerShipCam) 0.0 "VTBlend_Linear" 0.0 false)
          (Default|CallOnNewGameState "NewEnumerator6"))))))

(fn SpawnPlayerShip
  (bind _p_controller (Variables|PlayerComponents|GetP%20Controller))
  (bind _returnvalue (Game|SpawnActorfromClass "/Game/Star-Map/Blueprints/Ships/BP_PlayerShip.BP_PlayerShip_C" (Math|Transform|MakeTransform "0, 0, 0" "0, 0, 0" "1,1,1") "Undefined" 0 0))
  (bind _output_get (Variables|PlayerComponents|SetPlayerShip _returnvalue))
  (Utilities|IsValid _p_controller
    (:Is%20Valid
      (Pawn|Possess _p_controller _output_get)
      (bind _returnvalue_2 (Actor|GetActorOfClass "/Game/Star-Map/Blueprints/SceneActors/BP_ActorPlacer.BP_ActorPlacer_C"))
      (bind _output_get_2 (Variables|SceneACtor|SetplayerSpawner _returnvalue_2))
      (Utilities|IsValid _output_get_2
        (:Is%20Valid
          (Default|PlaceActor _output_get_2 (Variables|PlayerComponents|GetPlayerShip) true))
        (:Is%20Not%20Valid
          _))
      (Class|IInit|OnInit(Message) (Variables|PlayerComponents|GetPlayerShip))
      (Default|CallOnNewGameState "NewEnumerator3"))))

(fn SetUpHUD
  (Class|IPlayerController|SetUpHUD(Message) (Variables|PlayerComponents|GetP%20Controller))
  (Default|CallOnNewGameState "NewEnumerator9"))

(fn SetUpMinimapCamera
  (Utilities|IsValid (Variables|PlayerComponents|GetPlayerShip)
    (:Is%20Valid
      (bind _returnvalue (Game|SpawnActorfromClass "/Game/Star-Map/Blueprints/UX/BP_MinimapCamera.BP_MinimapCamera_C" (Math|Transform|MakeTransform "0, 0, 0" "0, 0, 0" "1,1,1") "Undefined" 0 "0.000000,0.000000,10000.000000" (Variables|PlayerComponents|GetPlayerShip) 6e+01 2e+03 2e+01 0))
      (bind _output_get (Variables|PlayerActors|SetMinimap%20Cam _returnvalue))
      (Default|Init _output_get)
      (Default|CallOnNewGameState "NewEnumerator7"))))

(fn BeginAsteroidGen
  (bind _returnvalue (Game|SpawnActorfromClass "/Game/Star-Map/Blueprints/Managers/BP_AsteroidGenerator.BP_AsteroidGenerator_C" (Math|Transform|MakeTransform "0, 0, 0" "0, 0, 0" "1,1,1") "Undefined" 0 0))
  (bind _output_get (Variables|SceneACtor|SetAsteroidGenerator _returnvalue))
  (CallFunction|OnBindtoAsteroidGen _output_get)
  (Default|Init (Variables|SceneACtor|GetAsteroidGenerator) "0, 0, 0" (Variables|MapDAta|GetMapRadius) (Variables|MapDAta|GetCluster%20Data))
  (Default|GenerateBoundary (Variables|SceneACtor|GetAsteroidGenerator)))

(fn AddLoadingScreen
  (Utilities|IsValid (Variables|UI|GetLoadingScreen)
    (:Is%20Valid
      (UserInterface|Viewport|AddtoViewport (Variables|UI|GetLoadingScreen) 0))
    (:Is%20Not%20Valid
      (bind _returnvalue (UserInterface|CreateWidget "/Game/Star-Map/Blueprints/Widget/W_Loading.W_Loading_C" (Game|GetPlayerController 0)))
      (bind _output_get (Variables|UI|SetLoadingScreen _returnvalue))
      (UserInterface|Viewport|AddtoViewport _output_get 0))))

(fn RemoveLoadingScreen
  (Utilities|IsValid (Variables|UI|GetLoadingScreen)
    (:Is%20Valid
      (Widget|RemovefromParent (Variables|UI|GetLoadingScreen)))))

(fn EvaluateScene
  (params (Scene :type E_Scenes%20Enum :default "NewEnumerator0"))
  (Class|IGameInstance|SetCurrentScene(Message) (Game|GetGameInstance) Scene)
  (switch Utilities|FlowControl|Switch|SwitchonE_Scenes Scene
    (:NewEnumerator0
      (return "L_MainMenu"))
    (:NewEnumerator1
      (return "L_Level1"))
    (:NewEnumerator3
      (return "L_Level2"))
    (:NewEnumerator4
      (return "L_Level3"))))

(fn TogglePause
  (if (Game|IsGamePaused)
    (Game|SetGamePaused false)
    (CallFunction|RemovePauseScreen)
    (else
      (Game|SetGamePaused true)
      (CallFunction|AddPauseScreeen))))

(fn SetIsGamePaused
  (params (bPaused :type Boolean))
  (Game|SetGamePaused bPaused))

(fn AddPauseScreeen
  (Utilities|IsValid (Variables|UI|GetPauseScreen)
    (:Is%20Valid
      (UserInterface|Viewport|AddtoViewport (Variables|UI|GetPauseScreen) 0))
    (:Is%20Not%20Valid
      (bind _returnvalue (UserInterface|CreateWidget "/Game/Star-Map/Blueprints/Widget/W_PauseScreen.W_PauseScreen_C" (Game|GetPlayerController 0)))
      (bind _output_get (Variables|UI|SetPauseScreen _returnvalue))
      (UserInterface|Viewport|AddtoViewport _output_get 0))))

(fn RemovePauseScreen
  (Utilities|IsValid (Variables|UI|GetPauseScreen)
    (:Is%20Valid
      (Widget|RemovefromParent (Variables|UI|GetPauseScreen)))))

(fn Init
  ;[1 1 1] Get all present actors with interface IInit
  (bind _outactors (Actor|GetAllActorswithInterface "/Game/Star-Map/Blueprints/Interfaces/I_Init.I_Init_C"))
  ;[1 1 1] Init them
  (for _array_element _outactors
    (Class|IInit|OnInit(Message) _array_element)
    ;[1 1 1] Login player
    (Default|CallOnNewGameState "NewEnumerator1")))

(fn StarGame
  (CallFunction|RemoveLoadingScreen)
  (Default|CallOnNewGameState "NewEnumerator10"))

(fn AddGameOverScreen
  (bind _returnvalue (UserInterface|CreateWidget "/Game/Star-Map/Blueprints/Widget/W_Gameover.W_Gameover_C" (Game|GetPlayerController 0)))
  (bind _output_get (Variables|Default|SetGameoverScreen _returnvalue))
  (UserInterface|Viewport|AddtoViewport _output_get 0))

(fn AddLevelSelectScreen
  (Utilities|IsValid (Variables|Default|GetLevelSelect)
    (:Is%20Valid
      (UserInterface|Viewport|AddtoViewport (Variables|Default|GetLevelSelect) 0))
    (:Is%20Not%20Valid
      (bind _returnvalue (UserInterface|CreateWidget "/Game/Star-Map/Blueprints/Widget/W_StarMap.W_StarMap_C" (Game|GetPlayerController 0)))
      (bind _output_get (Variables|Default|SetLevelSelect _returnvalue))
      (UserInterface|Viewport|AddtoViewport _output_get 0))))

(fn RemoveLevelSelectScreen
  (Utilities|IsValid (Variables|Default|GetLevelSelect)
    (:Is%20Valid
      (Widget|RemovefromParent (Variables|Default|GetLevelSelect)))))

(fn GetCanEndGame
  (return (Variables|GameState|GetCan%20End%20Game)))

(fn GetCurrentLevelName
  (bind _currentscenename (Class|IGameInstance|GetCurrentScene(Message) (Game|GetGameInstance)))
  (return (Utilities|String|EnumtoString _currentscenename)))

(fn GetStarMapGameMode
  (return self))