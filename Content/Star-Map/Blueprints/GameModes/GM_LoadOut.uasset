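; Game mode for the ship loadout screen, where the player fits weapons to four ports and buys from a shop.
; On BeginPlay it recreates the player controller, possesses the loadout ship, switches to the scene camera and fills the HUD from game instance data.
; Loadout changes update the HUD and ship, then save through the game instance, while purchases pass to the HUD.
; LoadScene saves again and opens the level mapped from the stored scene.
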(event EventBeginPlay
  (CallFunction|CreateNewController)
  (Utilities|FlowControl|Delay 0.2)
  (CallFunction|SetUpLoadOut)
  (CallFunction|AddHUD)
  (Variables|/Script/Engine.PlayerController|SetbShowMouseCursor (Game|GetPlayerController 0) true))

(event EventTick
  (params (DeltaSeconds :type Float%20%28single-precision%29)))

(event EventPostLogin
  (params (NewPlayer :type Player%20Controller%20Object%20Reference))
  ;[1 1 1] On Login
  (bind _aspc_load_out (Utilities|Casting|CastToPC_LoadOut NewPlayer))
  (Variables|Default|SetController _aspc_load_out))

(event EventBuyShopEntry
  (params (ShopIcon :type W%20Shop%20Icons%20Object%20Reference))
  (Default|BuyWeapon (Variables|Default|GetHUD) ShopIcon))

(event EventLoadScene
  (params (Scene :type E_Scenes%20Enum :default "NewEnumerator2"))
  (bind _returnvalue (Game|GetGameInstance))
  (bind _data (Class|IGameInstance|GetGameData(Message) _returnvalue))
  (Class|IGameInstance|SetGameData(Message) _returnvalue (Utilities|Struct|MakeS_StarmapData (.credits _data) (.levelscomplete _data) (Variables|Default|GetPlayer%20Ship%20Load%20Out) (.unlockedweapons _data) (.shop _data)))
  (Class|IGameInstance|OnSaveGame(Message) _returnvalue)
  (bind _currentscenename (Class|IGameInstance|GetCurrentScene(Message) (Game|GetGameInstance)))
  (bind _scenename (CallFunction|EvaluateScene _currentscenename))
  (Game|OpenLevel(byName) (Utilities|String|StringToName _scenename)))

(event EventOnLoadOutChanged
  (params (NewWeapon :type E_WeaponType%20Enum :default "NewEnumerator0") (WeaponPort :type E_PlayerModulePorts%20Enum :default "NewEnumerator0"))
  (bind _returnvalue (Game|GetGameInstance))
  (bind _hud (Variables|Default|GetHUD))
  (switch Utilities|FlowControl|Switch|SwitchonE_PlayerModulePorts WeaponPort
    (:NewEnumerator0
      (Default|OnNewWeaponAdded _hud (.weaponport0 (Variables|Default|GetPlayer%20Ship%20Load%20Out)))
      (Variables|Default|SetPlayer%20Ship%20Load%20Out (Utilities|Struct|MakeS_PlayerShipLoadOut NewWeapon (.weaponport1 (Variables|Default|GetPlayer%20Ship%20Load%20Out)) (.weaponport2 (Variables|Default|GetPlayer%20Ship%20Load%20Out)) (.weaponport3 (Variables|Default|GetPlayer%20Ship%20Load%20Out)))))
    (:NewEnumerator1
      (Default|OnNewWeaponAdded _hud (.weaponport1 (Variables|Default|GetPlayer%20Ship%20Load%20Out)))
      (Variables|Default|SetPlayer%20Ship%20Load%20Out (Utilities|Struct|MakeS_PlayerShipLoadOut (.weaponport0 (Variables|Default|GetPlayer%20Ship%20Load%20Out)) NewWeapon (.weaponport2 (Variables|Default|GetPlayer%20Ship%20Load%20Out)) (.weaponport3 (Variables|Default|GetPlayer%20Ship%20Load%20Out)))))
    (:NewEnumerator2
      (Default|OnNewWeaponAdded _hud (.weaponport2 (Variables|Default|GetPlayer%20Ship%20Load%20Out)))
      (Variables|Default|SetPlayer%20Ship%20Load%20Out (Utilities|Struct|MakeS_PlayerShipLoadOut (.weaponport0 (Variables|Default|GetPlayer%20Ship%20Load%20Out)) (.weaponport1 (Variables|Default|GetPlayer%20Ship%20Load%20Out)) NewWeapon (.weaponport3 (Variables|Default|GetPlayer%20Ship%20Load%20Out)))))
    (:NewEnumerator3
      (Default|OnNewWeaponAdded _hud (.weaponport3 (Variables|Default|GetPlayer%20Ship%20Load%20Out)))
      (Variables|Default|SetPlayer%20Ship%20Load%20Out (Utilities|Struct|MakeS_PlayerShipLoadOut (.weaponport0 (Variables|Default|GetPlayer%20Ship%20Load%20Out)) (.weaponport1 (Variables|Default|GetPlayer%20Ship%20Load%20Out)) (.weaponport2 (Variables|Default|GetPlayer%20Ship%20Load%20Out)) NewWeapon))))
  (Default|ReduceWeaponAvailable (Variables|Default|GetHUD) NewWeapon)
  (Default|SetWeaponPortbyEnum (Variables|Default|Getloadout) WeaponPort NewWeapon)
  (bind _data (Class|IGameInstance|GetGameData(Message) _returnvalue))
  (Class|IGameInstance|SetGameData(Message) _returnvalue (Utilities|Struct|MakeS_StarmapData (.credits _data) (.levelscomplete _data) (Variables|Default|GetPlayer%20Ship%20Load%20Out) (.unlockedweapons _data) (.shop _data)))
  (Class|IGameInstance|OnSaveGame(Message) _returnvalue))

(fn ConstructionScript)

(fn CreateNewController
  (Class|GameplayStatics|RemovePlayer (Game|GetPlayerController 0) true)
  (Class|GameplayStatics|CreatePlayer -1))

(fn SetUpLoadOut
  (bind _controller (Variables|Default|GetController))
  (bind _returnvalue (Actor|GetActorOfClass "/Game/Star-Map/Blueprints/VFX/Templates/BP_ShipLoadOut.BP_ShipLoadOut_C"))
  (bind _output_get (Variables|Default|Setloadout _returnvalue))
  (Default|Init _output_get)
  (Pawn|Possess _controller _output_get)
  (bind _returnvalue_2 (Actor|GetActorOfClass "/Game/Star-Map/Blueprints/UX/BP_MainMenuCamera.BP_MainMenuCamera_C"))
  (bind _output_get_2 (Variables|Default|SetSceneCamera _returnvalue_2))
  (Game|Player|SetViewTargetwithBlend _controller _output_get_2 0.0 "VTBlend_Linear" 0.0 false)
  (bind _data (Class|IGameInstance|GetGameData(Message) (Game|GetGameInstance)))
  (bind _output_get_3 (Variables|Default|SetGameData _data))
  (Variables|Default|SetPlayer%20Ship%20Load%20Out (.playershiploadout _output_get_3))
  (Default|SetUpEquippedWeapons (Variables|Default|Getloadout)))

(fn AddHUD
  (bind _returnvalue (UserInterface|CreateWidget "/Game/Star-Map/Blueprints/Widget/W_LoadOut.W_LoadOut_C"))
  (bind _output_get (Variables|Default|SetHUD _returnvalue))
  (UserInterface|Viewport|AddtoViewport _output_get 0)
  (bind _data (Class|IGameInstance|GetGameData(Message) (Game|GetGameInstance)))
  (Default|Init _output_get (.credits _data) (.playershiploadout _data) (.unlockedweapons _data) (.shop _data)))

(fn AddLoadingScreen
  (Utilities|IsValid (Variables|Default|GetLoadingScreen)
    (:Is%20Valid
      (UserInterface|Viewport|AddtoViewport (Variables|Default|GetLoadingScreen) 0))
    (:Is%20Not%20Valid
      (bind _returnvalue (UserInterface|CreateWidget "/Game/Star-Map/Blueprints/Widget/W_Loading.W_Loading_C" (Game|GetPlayerController 0)))
      (bind _output_get (Variables|Default|SetLoadingScreen _returnvalue))
      (UserInterface|Viewport|AddtoViewport _output_get 0))))

(fn RemoveLoadingScreen
  (Utilities|IsValid (Variables|Default|GetLoadingScreen)
    (:Is%20Valid
      (Widget|RemovefromParent (Variables|Default|GetLoadingScreen)))))

(fn EvaluateScene
  (params (Scene :type E_Scenes%20Enum :default "NewEnumerator0"))
  (Class|IGameInstance|SetCurrentScene(Message) (Game|GetGameInstance) Scene)
  (switch Utilities|FlowControl|Switch|SwitchonE_Scenes Scene
    (:NewEnumerator0
      (return "L_MainMenu"))
    (:NewEnumerator1
      (return "L_Level1"))
    (:NewEnumerator3
      (return "L_Level2"))
    (:NewEnumerator4
      (return "L_Level3"))))

(fn GetCanEndGame
  (return false))

(fn GetCurrentLevelName
  (return ""))

(fn GetStarMapGameMode
  (return 0))

(fn GetWeapon
  (return "NewEnumerator0"))