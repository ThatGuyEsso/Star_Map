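; GM_Testing is a test game mode that sets up a player ship with a top-down follow camera.
; On BeginPlay it removes the first local player and its pawn, then creates a fresh one, with PostLogin caching the latest controller.
; It then spawns a BP_BaseShip for that controller to possess and a BP_TopDownCamera that follows the ship from overhead as the view target.
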(event EventPostLogin
  (params (NewPlayer :type Player%20Controller%20Object%20Reference))
  ;[1 1 1] On Login
  (Variables|PlayerComponents|SetP%20Controller NewPlayer))

(event EventBeginPlay
  (CallFunction|CreateNewController)
  (CallFunction|SpawnPlayerShip)
  (CallFunction|SetUpPlayerCamera))

(fn ConstructionScript)

(fn CreateNewController
  (Class|GameplayStatics|RemovePlayer (Game|GetPlayerController 0) true)
  (Class|GameplayStatics|CreatePlayer -1))

(fn SetUpPlayerCamera
  (bind _p_controller (Variables|PlayerComponents|GetP%20Controller))
  (Utilities|IsValid (Variables|PlayerComponents|GetPlayerShip)
    (:Is%20Valid
      (bind _returnvalue (Game|SpawnActorfromClass "/Game/Star-Map/Blueprints/UX/BP_TopDownCamera.BP_TopDownCamera_C" (Math|Transform|MakeTransform "0, 0, 0" "0, 0, 0" "1,1,1") "Undefined" 0 "0.000000,0.000000,2850.000000" (Variables|PlayerComponents|GetPlayerShip) 5.0 0))
      (bind _output_get (Variables|PlayerComponents|SetPlayerShipCam _returnvalue))
      (Default|Init _output_get)
      (Utilities|IsValid _p_controller
        (:Is%20Valid
          (Game|Player|SetViewTargetwithBlend _p_controller (Variables|PlayerComponents|GetPlayerShipCam) 0.0 "VTBlend_Linear" 0.0 false))))))

(fn SpawnPlayerShip
  (bind _p_controller (Variables|PlayerComponents|GetP%20Controller))
  (bind _returnvalue (Game|SpawnActorfromClass "/Game/Star-Map/Blueprints/Ships/BP_BaseShip.BP_BaseShip_C" (Math|Transform|MakeTransform "0.000000,0.000000,600.000000" "0, 0, 0" "1,1,1") "Undefined" 0 0))
  (bind _output_get (Variables|PlayerComponents|SetPlayerShip _returnvalue))
  (Utilities|IsValid _p_controller
    (:Is%20Valid
      (Pawn|Possess _p_controller _output_get))))