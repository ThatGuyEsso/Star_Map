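; Minimap camera actor that follows a target at a set offset and changes height with the target's movement.
; Init positions it, aims it at the target once and binds to the target's RigidBodyMessage accelerating and stopping events.
; Tick interpolates toward the offset position, then zooms by moving Z: up by a speed-percent amount while moving, slowly back when stopped.
; MaxZoomOut is computed in Init but never applied here.
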(event Custom|OnBindToMovement
  (bind _target (Variables|FollowSettings|Gettarget))
  (Utilities|IsValid _target
    (:Is%20Valid
      (bind _rigidbody (Class|ISpaceShip|GetRigidBody(Message) _target))
      (Utilities|IsValid _rigidbody
        (:Is%20Valid
          (EventDispatchers|BindEventtoOnAccelerating _rigidbody (delegate Custom|OnZoomOut))
          (EventDispatchers|BindEventtoOnStopping _rigidbody (delegate Custom|OnZoomIn)))))))

(event Custom|OnZoomOut
  (params (percentSpeed :type Float%20%28single-precision%29))
  (Variables|State|SetisTargetMoving true)
  (Variables|FollowSettings|SettargetPecentZoom percentSpeed))

(event Custom|OnZoomIn
  (params (PercentSpeed :type Float%20%28single-precision%29))
  (Variables|State|SetisTargetMoving false)
  (Variables|FollowSettings|SettargetPecentZoom PercentSpeed))

(event EventTick
  (params (DeltaSeconds :type Float%20%28single-precision%29))
  (if (Variables|State|GetIsFollowing)
    (Utilities|IsValid (Variables|FollowSettings|Gettarget)
      (:Is%20Valid
        (Transformation|SetActorLocation (Math|Interpolation|VInterpTo (Transformation|GetActorLocation) (+ (Transformation|GetActorLocation (Variables|FollowSettings|Gettarget)) (Variables|FollowSettings|GetOffSetToTarget)) DeltaSeconds (Variables|FollowSettings|GetFollowRate)) false false)
        (if (Variables|State|GetisTargetMoving)
          (CallFunction|Zoom DeltaSeconds (+ (* (Variables|FollowSettings|GetFlightZoomOutAmount) (Variables|FollowSettings|GettargetPecentZoom)) (.z (Transformation|GetActorLocation))) (Variables|FollowSettings|GetZoomRate))
          (else
            (CallFunction|Zoom DeltaSeconds (+ (.z (Transformation|GetActorLocation (Variables|FollowSettings|Gettarget))) (.z (Variables|FollowSettings|GetOffSetToTarget))) 0.01)))))))

(fn ConstructionScript)

(fn SetIsFollowTarget
  (params (IsFollowing :type Boolean))
  (Variables|State|SetIsFollowing IsFollowing))

(fn SetFollowTarget
  (params (target :type Actor%20Object%20Reference))
  (Variables|FollowSettings|Settarget target))

(fn Init
  (Utilities|IsValid (Variables|FollowSettings|Gettarget)
    (:Is%20Valid
      (Transformation|SetActorLocation (+ (Transformation|GetActorLocation (Variables|FollowSettings|Gettarget)) (Variables|FollowSettings|GetOffSetToTarget)) false false)
      (Transformation|SetActorRotation (Math|Rotator|FindLookatRotation (Transformation|GetActorLocation) (Transformation|GetActorLocation (Variables|FollowSettings|Gettarget))))
      (Variables|State|SetIsFollowing true)
      (Variables|FollowSettings|SetMaxZoomOut (+ (.z (Variables|FollowSettings|GetOffSetToTarget)) (Variables|FollowSettings|GetMaxZoomOut)))
      (CallFunction|OnBindtoMovement))))

(fn Zoom
  (params (DeltaTime :type Float%20%28single-precision%29) (Target%20Zoom :type Float%20%28single-precision%29) (InterpSpeed :type Float%20%28single-precision%29))
  (bind _returnvalue (Transformation|GetActorLocation))
  (Transformation|SetActorLocation (Math|Interpolation|VInterpTo (Transformation|GetActorLocation) (Math|Vector|MakeVector (.x _returnvalue) (.y _returnvalue) Target%20Zoom) DeltaTime InterpSpeed) false false))