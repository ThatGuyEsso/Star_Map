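; Game instance for the Star-Map game that holds current game data and level, and manages the SG_StarmapSave slot.
; It loads or creates the save object on Init, and writes GameData into it on Shutdown or OnSaveGame.
; Loading never copies saved data back into GameData, and only OnLoadGame sets HasExistingSave.
; Scene changes update the level number, mapped only for Level One; ResetData and GetGameData are empty stubs.
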(event EventInit
  (CallFunction|LoadData))

(event EventShutdown
  (CallFunction|SaveData))

(event EventOnSaveGame
  (CallFunction|SaveData))

(event EventOnLoadGame
  (bind _hassave (CallFunction|LoadData))
  (Variables|Default|SetHasExistingSave _hassave))

(event EventSetCurrentScene
  (params (CurrentScene :type E_Scenes%20Enum :default "NewEnumerator2"))
  (Variables|Default|SetCurrentLevel CurrentScene)
  (CallFunction|EvaluateNumber))

(event EventSetGameData
  (params (Data :type S%20Starmap%20Game%20Data%20Structure))
  (Variables|Default|SetGameData Data))

(fn SaveData
  (bind _currentsave (Variables|Default|GetCurrentSave))
  (Variables|/Game/Star-Map/Blueprints/Data/SG_StarmapSave.SG_StarmapSave_C|SetSaveData _currentsave (Variables|Default|GetGameData))
  (SaveGame|SaveGametoSlot _currentsave (Variables|Default|GetSlot%20Name)))

(fn LoadData
  (bind _returnvalue (SaveGame|DoesSaveGameExist (Variables|Default|GetSlot%20Name)))
  (if _returnvalue
    (bind _returnvalue_2 (SaveGame|LoadGamefromSlot (Variables|Default|GetSlot%20Name)))
    (bind _assg_starmap_save (Utilities|Casting|CastToSG_StarmapSave _returnvalue_2))
    (Variables|Default|SetCurrentSave _assg_starmap_save)
    (return true)
    (else
      (bind _returnvalue_3 (SaveGame|CreateSaveGameObject "/Game/Star-Map/Blueprints/Data/SG_StarmapSave.SG_StarmapSave_C"))
      (Variables|Default|SetCurrentSave _returnvalue_3)
      (return false))))

(fn ResetData)

(fn EvaluateNumber
  (switch Utilities|FlowControl|Switch|SwitchonE_Scenes (Variables|Default|GetCurrentLevel)
    (:NewEnumerator1
      (Variables|Default|SetCurrentLevelNumber 1))))

(fn GetCurrentLevelNumber
  (return (Variables|Default|GetCurrentLevelNumber)))

(fn GetCurrentScene
  (return (Variables|Default|GetCurrentLevel)))

(fn GetGameData
  (return ""))

(fn HasExisitingSave
  (return (Variables|Default|GetHasExistingSave)))