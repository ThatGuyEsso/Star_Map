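; BP_BeamConnector is a VFX actor in the Star-Map content that draws a particle beam between a source actor and a target actor.
; BeginPlay applies the particle template, and Init sets the beam endpoints once from both actors' locations, without tracking movement.
; Init also binds both actors' destruction to ClearEmitter, which pushes the endpoints to a hugely scaled, far-off position before destroying the connector.
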(event Custom|BindToOnDestroy
  (Game|BindEventtoOnDestroyed (Variables|Default|GetSourceACtor) (delegate Custom|OnClear))
  (Game|BindEventtoOnDestroyed (Variables|Default|GetTargetActor) (delegate Custom|OnClear)))

(event Custom|OnClear
  (params (DestroyedActor :type Actor%20Object%20Reference))
  (CallFunction|ClearEmitter))

(event EventBeginPlay
  (Effects|Components|ParticleSystem|SetTemplate (Variables|Default|GetParticleSystem) (Variables|Default|GetParticleTemplate)))

(event Collision|EventActorBeginOverlap
  (params (OtherActor :type Actor%20Object%20Reference)))

(event EventTick
  (params (DeltaSeconds :type Float%20%28single-precision%29)))

(fn ConstructionScript)

(fn ClearEmitter
  (bind _returnvalue (Transformation|GetActorLocation))
  (bind _particlesystem (Variables|Default|GetParticleSystem))
  (bind _returnvalue_2 (* _returnvalue 1e+07))
  ;[1 1 1] Remove and destroy component
  (Class|ParticleSystemComponent|SetBeamTargetPoint _particlesystem 0 _returnvalue_2)
  (Class|ParticleSystemComponent|SetBeamSourcePoint _particlesystem 0 _returnvalue_2)
  (Actor|DestroyActor))

(fn Init
  (params (SourceACtor :type Actor%20Object%20Reference) (TargetActor :type Actor%20Object%20Reference))
  (bind _particlesystem (Variables|Default|GetParticleSystem))
  (bind _output_get (Variables|Default|SetSourceACtor SourceACtor))
  (bind _output_get_2 (Variables|Default|SetTargetActor TargetActor))
  (Utilities|IsValid _output_get
    (:Is%20Valid
      (Utilities|IsValid _output_get_2
        (:Is%20Valid
          (Class|ParticleSystemComponent|SetBeamSourcePoint _particlesystem 0 (Transformation|GetActorLocation _output_get))
          (Class|ParticleSystemComponent|SetBeamTargetPoint _particlesystem 0 (Transformation|GetActorLocation _output_get_2))
          (CallFunction|BindtoonDestroy))))))