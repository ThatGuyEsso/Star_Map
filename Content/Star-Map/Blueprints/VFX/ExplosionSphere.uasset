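; ExplosionSphere is a short-lived VFX actor in the star map that shows a coloured explosion sphere.
; InitSphere sets its world scale, position and lifetime, and tints the sphere through a dynamic material instance's FlashCol parameter.
; It then calls OnDelete, which waits for the stored Duration and destroys the actor.
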(event Custom|OnDelete
  (Utilities|FlowControl|Delay (Variables|Default|GetDuration))
  (Actor|DestroyActor))

(fn ConstructionScript)

(fn InitSphere
  (params (Scale :type Float%20%28single-precision%29) (Duration :type Float%20%28single-precision%29) (Colour :type Linear%20Color%20Structure) (position :type Vector))
  (Transformation|SetWorldScale3D (Variables|Default|GetDefaultSceneRoot) (Math|Conversions|ToVector(Float) Scale))
  (Variables|Default|SetDuration Duration)
  (bind _returnvalue (Rendering|Material|CreateDynamicMaterialInstance (Variables|Default|GetSphere) 0 (Rendering|Material|GetMaterial (Variables|Default|GetSphere) 0) "None" :!class /Script/Engine.PrimitiveComponent))
  (Rendering|Material|SetVectorParameterValue _returnvalue "FlashCol" Colour :!class /Script/Engine.MaterialInstanceDynamic)
  (Transformation|SetActorLocation position false false)
  (CallFunction|OnDelete))