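; Explosion VFX manager that creates a randomized burst of explosion spheres and sound at its location on BeginPlay, then destroys itself.
; GenerateExplosion spawns a random number of ExplosionSphere actors, initializing each with a random scale, duration, color and positional offset from the Settings ranges and palette.
; PlayExplosionSFX hands the sound to a separately spawned BP_AudioPlayer with random pitch before the manager is destroyed.
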(event EventBeginPlay
  (CallFunction|GenerateExplosion))

(event Collision|EventActorBeginOverlap
  (params (OtherActor :type Actor%20Object%20Reference)))

(event EventTick
  (params (DeltaSeconds :type Float%20%28single-precision%29)))

(fn ConstructionScript)

(fn GenerateExplosion
  (bind _settings (Variables|Default|GetSettings))
  (bind _settings_2 (Variables|Default|GetSettings))
  (bind _settings_3 (Variables|Default|GetSettings))
  (bind _output_get (LocalVariables|SetnToSPawn (Math|Random|RandomIntegerinRange (.mintospawn _settings_3) (.maxtospawn _settings_3))))
  (for _index (range 0 (- _output_get 1))
    (bind _returnvalue (Game|SpawnActorfromClass "/Game/Star-Map/Blueprints/VFX/ExplosionSphere.ExplosionSphere_C" (Math|Transform|MakeTransform "0, 0, 0" "0, 0, 0" "1,1,1") "Undefined" 0 0))
    (Utilities|Array|Add (LocalVariables|Getexplosions) _returnvalue))
  (for _array_element (LocalVariables|Getexplosions)
    (Default|InitSphere _array_element (Math|Random|RandomFloatinRange (.minsize _settings_2) (.maxsize _settings_2)) (Math|Random|RandomFloatinRange (.minduration _settings_2) (.maxduration _settings_2)) (Utilities|Array|Get(acopy) (.expolsioncolours _settings_2) (Math|Random|RandomIntegerinRange 0 (Utilities|Array|LastIndex (.expolsioncolours _settings_2)))) (+ (Transformation|GetActorLocation) (Math|Vector|MakeVector (Math|Random|RandomFloatinRange (.minoffset _settings) (.maxoffset _settings)) (Math|Random|RandomFloatinRange (.minoffset _settings) (.maxoffset _settings)) (Math|Random|RandomFloatinRange (.minoffset _settings) (.maxoffset _settings))))))
  (CallFunction|PlayExplosionSFX)
  (Actor|DestroyActor))

(fn PlayExplosionSFX
  (bind _returnvalue (Game|SpawnActorfromClass "/Game/Star-Map/Blueprints/UX/BP_AudioPlayer.BP_AudioPlayer_C" (Math|Transform|MakeTransform (Transformation|GetActorLocation) "0, 0, 0" "1,1,1") "Undefined" 0 (Variables|Default|GetExplosionSFX) true false false 3.0 0))
  (Default|PlaySound _returnvalue))