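; Star-map manager that spawns asteroid clusters around a cached origin and fills them with asteroids.
; GenerateClusters spawns the configured number of BP_AsteroidCluster actors with random radii, using only X and Y of random points in the bounds.
; GenerateAsteroids then has each cluster spawn its asteroids from the generation data and signals completion.
; Despite the "sphere" naming, random points and the IsWithinRange check use an axis-aligned box.
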(event EventBeginPlay)

(event Collision|EventActorBeginOverlap
  (params (OtherActor :type Actor%20Object%20Reference)))

(event EventTick
  (params (DeltaSeconds :type Float%20%28single-precision%29)))

(fn ConstructionScript)

(fn Init
  (params (Orgin :type Vector) (radius :type Float%20%28single-precision%29) (ClusterData :type S%20Asteroid%20Cluster%20Gen%20Data%20Structure))
  ;[1 1 1] Cache data
  (Variables|Default|SetOrgin Orgin)
  (Variables|Default|SetRadius radius)
  (Variables|Default|SetCluster%20Data ClusterData))

(fn IsWithinRange
  (params (point :type Vector))
  (LocalVariables|SetdesiredPoint point)
  (LocalVariables|SetminExtent (- (Variables|Default|GetOrgin) (* (Class|KismetMathLibrary|VectorOne) (Variables|Default|GetRadius))))
  (LocalVariables|SetMaxExtent (+ (Variables|Default|GetOrgin) (* (Class|KismetMathLibrary|VectorOne) (Variables|Default|GetRadius))))
  ;[1 1 1] Returns result
  (return (Math|Boolean|ANDBoolean (and (>= (.x (LocalVariables|GetdesiredPoint)) (.x (LocalVariables|GetminExtent))) (<= (.x (LocalVariables|GetdesiredPoint)) (.x (LocalVariables|GetMaxExtent)))) (and (>= (.y (LocalVariables|GetdesiredPoint)) (.y (LocalVariables|GetminExtent))) (<= (.y (LocalVariables|GetdesiredPoint)) (.y (LocalVariables|GetMaxExtent)))) (and (>= (.z (LocalVariables|GetdesiredPoint)) (.z (LocalVariables|GetminExtent))) (<= (.z (LocalVariables|GetdesiredPoint)) (.z (LocalVariables|GetMaxExtent)))))))

(fn GenerateClusters
  (bind _cluster_data (Variables|Default|GetCluster%20Data))
  ;[1 1 1] Try and Generate max clusters by running it max times
  (for _index (range 0 (- (.maxclusters (Variables|Default|GetCluster%20Data)) 1))
    (bind _point (CallFunction|GetRandomPointinSphereRange))
    (bind _output_get (LocalVariables|SetRandomPoint _point))
    (bind _returnvalue (Game|SpawnActorfromClass "/Game/Star-Map/Blueprints/Props/BP_AsteroidCluster.BP_AsteroidCluster_C" (Math|Transform|MakeTransform (Math|Vector|MakeVector (.x _output_get) (.y _output_get) 0.0) "0, 0, 0" "1,1,1") "Undefined" 0 (Math|Random|RandomFloatinRange (.maxclustersize _cluster_data) (.minclustersize _cluster_data)) 0))
    (LocalVariables|SetcurrentCluster _returnvalue)
    (Utilities|Array|Add (Variables|Default|GetClusters) (LocalVariables|GetcurrentCluster)))
  (CallFunction|GenerateAsteroids))

(fn GetRandomPointinSphereRange
  (LocalVariables|SetminExtent (- (Variables|Default|GetOrgin) (* (Class|KismetMathLibrary|VectorOne) (Variables|Default|GetRadius))))
  (LocalVariables|SetMaxExtent (+ (Variables|Default|GetOrgin) (* (Class|KismetMathLibrary|VectorOne) (Variables|Default|GetRadius))))
  (return (Math|Vector|MakeVector (Math|Random|RandomFloatinRange (.x (LocalVariables|GetminExtent)) (.x (LocalVariables|GetMaxExtent))) (Math|Random|RandomFloatinRange (.y (LocalVariables|GetminExtent)) (.y (LocalVariables|GetMaxExtent))) (Math|Random|RandomFloatinRange (.z (LocalVariables|GetminExtent)) (.z (LocalVariables|GetMaxExtent))))))

(fn GenerateAsteroids
  (if (> (Utilities|Array|Length (Variables|Default|GetClusters)) 0)
    (for _array_element (Variables|Default|GetClusters)
      (Default|SpawnAsteroids _array_element (.astroidgendata (Variables|Default|GetCluster%20Data))))
    (Default|CallOnAsteroidGenComplete)))