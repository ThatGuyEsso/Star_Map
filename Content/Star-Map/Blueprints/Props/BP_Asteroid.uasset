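; BP_Asteroid is a rotating asteroid prop with a randomized appearance and a minimap icon.
; Init picks a random mesh and material, randomizes the RotatingMovement rate within MaxRotation, and spawns BP_MiniMapIcon at its location.
; CanBePlaced uses a multi sphere trace at the scaled collision radius, testing hit actors against asteroid and player ship classes.
; A collision hit handler is meant to flag asteroid-on-asteroid contact.
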(event OnComponentHit(Collision)
  (params (HitComponent :type Primitive%20Component%20Object%20Reference) (OtherActor :type Actor%20Object%20Reference) (OtherComp :type Primitive%20Component%20Object%20Reference) (NormalImpulse :type Vector :default "0, 0, 0") (Hit :type Hit%20Result%20Structure%20%28by%20ref%29))
  (bind _returnvalue (Components|GetOwner HitComponent))
  (bind _self self)
  (if (!= _returnvalue _self)
    (if (== (Utilities|GetClass _returnvalue) (Utilities|GetClass _self))
      (Variables|Default|SetIsInAsteroidCOllision true))))

(event EventBeginPlay)

(event Collision|EventActorBeginOverlap
  (params (OtherActor :type Actor%20Object%20Reference)))

(event EventTick
  (params (DeltaSeconds :type Float%20%28single-precision%29)))

(fn ConstructionScript)

(fn CanbePlaced
  (bind _returnvalue (Transformation|GetActorLocation))
  (bind _outhits (Collision|MultiSphereTraceByChannel _returnvalue _returnvalue (* (Variables|/Script/Engine.SphereComponent|GetSphereRadius (Variables|Default|GetCollision)) (.x (Transformation|GetActorScale3D))) "TraceTypeQuery1" false 0 "None"))
  (for _array_element _outhits
    (if (.bblockinghit _array_element)
      (return true)
      (elif (!= (Components|GetOwner (.hitcomponent _array_element)) self)
        (return (and (!= (Utilities|GetClass (Components|GetOwner (.hitcomponent _array_element))) "BP_Asteroid_C") (!= (Utilities|GetClass (Components|GetOwner (.hitcomponent _array_element))) "/Game/Star-Map/Blueprints/Ships/BP_PlayerShip.BP_PlayerShip_C")))
        (else
          (return true))))))

(fn RandomStaticMesh
  (bind _possiblemeshes (Variables|Default|GetPossibleMEshes))
  (Components|StaticMesh|SetStaticMesh (Variables|Default|GetStaticMesh) (Utilities|Array|Get(acopy) _possiblemeshes (Math|Random|RandomIntegerinRange 0 (Utilities|Array|LastIndex _possiblemeshes)))))

(fn Init
  (bind _maxrotation (Variables|Default|GetMaxRotation))
  (bind _defaultsceneroot (Variables|Default|GetDefaultSceneRoot))
  (CallFunction|RandomStaticMesh)
  (CallFunction|RandomMeshMaterial)
  (Variables|/Script/Engine.RotatingMovementComponent|SetRotationRate (Variables|Default|GetRotatingMovement) (Math|Rotator|MakeRotator (Math|Random|RandomFloatinRange (* -1 (.x _maxrotation)) (.x _maxrotation)) (Math|Random|RandomFloatinRange (* -1 (.y _maxrotation)) (.y _maxrotation)) (Math|Random|RandomFloatinRange (* -1 (.z _maxrotation)) (.z _maxrotation))))
  (Game|SpawnActorfromClass "/Game/Star-Map/Blueprints/UX/BP_MiniMapIcon.BP_MiniMapIcon_C" (Math|Transform|MakeTransform (Transformation|GetWorldLocation _defaultsceneroot) "0, 0, 0" (Transformation|GetWorldScale _defaultsceneroot)) "Undefined" 0 0))

(fn RandomMeshMaterial
  (bind _possiblematerials (Variables|Default|GetPossibleMaterials))
  (Rendering|Material|SetMaterial (Variables|Default|GetStaticMesh) 0 (Utilities|Array|Get(acopy) _possiblematerials (Math|Random|RandomIntegerinRange 0 (Utilities|Array|LastIndex _possiblematerials)))))