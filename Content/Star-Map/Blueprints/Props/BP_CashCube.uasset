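; Cash pickup prop that spins at a random rate and flies to the player when they come near.
; The Sphere overlap locks onto the Player-tagged actor, and Tick then sweeps the cube toward it while the pull speed eases up to MaxForce.
; Touching the Box sends a fixed cash amount to the game mode through OnAddCashMessage and destroys the cube.
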(event OnComponentBeginOverlap(Sphere)
  (params (OverlappedComponent :type Primitive%20Component%20Object%20Reference) (OtherActor :type Actor%20Object%20Reference) (OtherComp :type Primitive%20Component%20Object%20Reference) (OtherBodyIndex :type Integer) (bFromSweep :type Boolean) (SweepResult :type Hit%20Result%20Structure%20%28by%20ref%29))
  (bind _returnvalue (Components|GetOwner OtherComp))
  (if (and (Actor|ActorHasTag _returnvalue "Player") (not (Variables|Default|GetMovingToPlayer)))
    (Variables|Default|SetMovingToPlayer true)
    (Variables|Default|SetTarget _returnvalue)))

(event OnComponentBeginOverlap(Box)
  (params (OverlappedComponent :type Primitive%20Component%20Object%20Reference) (OtherActor :type Actor%20Object%20Reference) (OtherComp :type Primitive%20Component%20Object%20Reference) (OtherBodyIndex :type Integer) (bFromSweep :type Boolean) (SweepResult :type Hit%20Result%20Structure%20%28by%20ref%29))
  (if (Actor|ActorHasTag (Components|GetOwner OtherComp) "Player")
    (Class|IGameMode|OnAddCash(Message) (Game|GetGameMode) 1e+01)
    (Actor|DestroyActor)))

(event EventBeginPlay
  (bind _rand (Variables|Default|GetRand))
  (bind _returnvalue (* _rand -1.0))
  (Variables|/Script/Engine.RotatingMovementComponent|SetRotationRate (Variables|Default|GetRotatingMovement) (Math|Rotator|MakeRotator (Math|Random|RandomFloatinRange _returnvalue _rand) (Math|Random|RandomFloatinRange _returnvalue _rand) (Math|Random|RandomFloatinRange _returnvalue _rand)))
  (Utilities|FlowControl|Delay 0.2))

(event Collision|EventActorBeginOverlap
  (params (OtherActor :type Actor%20Object%20Reference)))

(event EventTick
  (params (DeltaSeconds :type Float%20%28single-precision%29))
  (if (Variables|Default|GetMovingToPlayer)
    (Utilities|IsValid (Variables|Default|GetTarget)
      (:Is%20Valid
        (Transformation|SetActorLocation (Math|Interpolation|VInterptoConstant (Transformation|GetActorLocation) (Transformation|GetActorLocation (Variables|Default|GetTarget)) DeltaSeconds (Variables|Default|GetForce)) true false)
        (Variables|Default|SetForce (Math|Interpolation|FInterpTo (Variables|Default|GetForce) (Variables|Default|GetMaxForce) DeltaSeconds 1e+01))))))

(fn ConstructionScript)