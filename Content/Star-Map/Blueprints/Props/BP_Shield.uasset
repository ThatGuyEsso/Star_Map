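; Shield actor that forwards damage to its owner and can be enabled or disabled, toggling collision and visibility and spawning an attached on/off sound.
; As a follower, it moves each tick to the owner's velocity-predicted next-frame location and copies its rotation.
; FlashOn swaps in a hurt material tinted by health ratio, and Tick counts down the timer until FlashOff restores the default material.
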(event EventBeginPlay
  (Variables|Default|SetdefaultMaterial (Rendering|Material|GetMaterial (Variables|Default|GetShieldMesh) 0)))

(event EventTick
  (params (DeltaSeconds :type Float%20%28single-precision%29))
  (bind _returnvalue (Components|GetOwner))
  ;[1 1 1] FlashTimer
  (if (Variables|Default|GetIsFlashing)
    (bind _output_get (Variables|Default|SetCurrentFlashTime (- (Variables|Default|GetCurrentFlashTime) DeltaSeconds)))
    (if (<= _output_get 0.0)
      (CallFunction|FlashOff)))
  ;[1 1 1] If owner is not stationary
  (if (Variables|Default|GetIsFollower)
    (Utilities|IsValid _returnvalue
      (:Is%20Valid
        ;[1 1 1] Update location rotation
        (Transformation|SetActorLocation (+ (Transformation|GetActorLocation _returnvalue) (* (Transformation|GetVelocity _returnvalue) DeltaSeconds)) true false)
        (Transformation|SetActorRotation (Transformation|GetActorRotation _returnvalue))))))

(event EventApplyDamage
  (params (Damage :type Float%20%28single-precision%29) (Instigator :type Actor%20Object%20Reference))
  ;[1 1 1] OnDamage
  (Class|IDamage|ApplyDamage(Message) (Components|GetOwner) Damage Instigator))

(fn ConstructionScript)

(fn DoDamageFlash)

(fn Flashon
  (params (CurrentHealth :type Float%20%28single-precision%29) (MaxHealth :type Float%20%28single-precision%29) (FlashTime :type Float%20%28single-precision%29))
  (bind _returnvalue (/ CurrentHealth MaxHealth))
  (bind _shieldmesh (Variables|Default|GetShieldMesh))
  (Variables|Default|SetCurrentFlashTime FlashTime)
  (Utilities|IsValid _shieldmesh
    (:Is%20Valid
      (bind _returnvalue_2 (Rendering|Material|CreateDynamicMaterialInstance _shieldmesh 0 (Variables|Default|GethurtMat) "None" :!class /Script/Engine.PrimitiveComponent))
      (bind _returnvalue_3 (Rendering|Material|GetVectorParameterValue _returnvalue_2 "FlashCol" :!class /Script/Engine.MaterialInstanceDynamic))
      (bind _output_get (LocalVariables|SetFlashColour _returnvalue_3))
      (bind _output_get_2 (Variables|Default|SetflashTint (Utilities|Struct|MakeLinearColor (/ (.r _output_get) _returnvalue) (* (.g _output_get) _returnvalue) (* (.b _output_get) _returnvalue) (.a _output_get))))
      (Rendering|Material|SetVectorParameterValue _returnvalue_2 "FlashCol" _output_get_2 :!class /Script/Engine.MaterialInstanceDynamic)
      (Variables|Default|SetIsFlashing true))))

(fn FlashOff
  (bind _shieldmesh (Variables|Default|GetShieldMesh))
  (Utilities|IsValid _shieldmesh
    (:Is%20Valid
      (Rendering|Material|CreateDynamicMaterialInstance _shieldmesh 0 (Variables|Default|GetdefaultMaterial) "None" :!class /Script/Engine.PrimitiveComponent)
      (Variables|Default|SetIsFlashing false))))

(fn DisableShield
  (Collision|SetCollisionEnabled (Variables|Default|GetSphere) "NoCollision")
  (Rendering|SetVisibility (Variables|Default|GetShieldMesh) false false)
  (Variables|Default|SetIsEnabled false)
  (bind _returnvalue (Game|SpawnActorfromClass "/Game/Star-Map/Blueprints/UX/BP_AudioPlayer.BP_AudioPlayer_C" (Math|Transform|MakeTransform (Transformation|GetActorLocation) "0, 0, 0" "1,1,1") "Undefined" 0 (Variables|Default|GetShieldOffSFX) true false false 3.0 0))
  (Utilities|IsValid _returnvalue
    (:Is%20Valid
      (Transformation|AttachActorToActor _returnvalue self "None" "KeepRelative" "KeepRelative" "KeepRelative" false))))

(fn EnableShield
  (bind _self self)
  (Collision|SetCollisionEnabled (Variables|Default|GetSphere) "QueryAndPhysics")
  (Rendering|SetVisibility (Variables|Default|GetShieldMesh) true false)
  (Variables|Default|SetIsEnabled true)
  (bind _returnvalue (Game|SpawnActorfromClass "/Game/Star-Map/Blueprints/UX/BP_AudioPlayer.BP_AudioPlayer_C" (Math|Transform|MakeTransform (Transformation|GetActorLocation (Components|GetOwner)) "0, 0, 0" "1,1,1") "Undefined" 0 (Variables|Default|GetShieldOnSFX) true false false 3.0 0))
  (Utilities|IsValid _self
    (:Is%20Valid
      (Utilities|IsValid _returnvalue
        (:Is%20Valid
          (Transformation|AttachActorToActor _returnvalue _self "None" "KeepRelative" "KeepRelative" "KeepRelative" false))))))

(fn IsShieldEnabled
  (return (Variables|Default|GetIsEnabled)))