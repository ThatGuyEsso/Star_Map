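; BP_ActorPlacer is a Star-Map scene actor that teleports a supplied actor to one of its spawn points.
; PlaceActor optionally copies the placer's rotation, then picks a random VectorSpawnPoints entry, added to the placer's location as an unrotated offset.
; With no spawn points, it sets the placer's own location to itself, so the supplied actor is not moved.
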(event EventBeginPlay)

(event Collision|EventActorBeginOverlap
  (params (OtherActor :type Actor%20Object%20Reference)))

(event EventTick
  (params (DeltaSeconds :type Float%20%28single-precision%29)))

(fn ConstructionScript)

(fn PlaceActor
  (params (actorToPlace :type Actor%20Object%20Reference) (matchSpawnPointRotation :type Boolean))
  (bind _returnvalue (Transformation|GetActorLocation))
  (if matchSpawnPointRotation
    (Transformation|SetActorRotation actorToPlace (Transformation|GetActorRotation) true))
  (if (> (Utilities|Array|Length (Variables|Default|GetVectorSpawnPoints)) 0)
    (bind _output_get (LocalVariables|SetspawnPoint (+ (Utilities|Array|Get(acopy) (Variables|Default|GetVectorSpawnPoints) (Math|Random|RandomIntegerinRange 0 (Utilities|Array|LastIndex (Variables|Default|GetVectorSpawnPoints)))) _returnvalue)))
    (Transformation|SetActorLocation actorToPlace _output_get false true)
    (else
      (Transformation|SetActorLocation _returnvalue false true))))