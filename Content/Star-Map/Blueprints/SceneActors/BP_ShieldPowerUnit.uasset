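; BP_ShieldPowerUnit is a Star-Map scene actor for a shield power unit with its own shield and hull health, marked as an objective on the minimap.
; Init extends the parent's setup by initialising BPCShieldAndHealth with a scaled solid shield.
; ApplyDamage forwards to that component's OnDamageTaken, always passing zero damage.
; SpawnMiniMapIcon spawns a BP_MiniMapIcon with the objective sprite at the root's location.
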(event EventBeginPlay
  (|CallParentFunction) ; This node is disabled and will not be called.\nDrag off pins to build functionality.
)

(event Collision|EventActorBeginOverlap
  (params (OtherActor :type Actor%20Object%20Reference))
  (|CallParentFunction OtherActor) ; This node is disabled and will not be called.\nDrag off pins to build functionality.
)

(event EventTick
  (params (DeltaSeconds :type Float%20%28single-precision%29))
  (|CallParentFunction DeltaSeconds) ; This node is disabled and will not be called.\nDrag off pins to build functionality.
)

(event EventApplyDamage
  (params (Damage :type Float%20%28single-precision%29) (Instigator :type Actor%20Object%20Reference))
  (Default|OnDamageTaken (Variables|Default|GetBPC_Shield_And_Health) 0.0))

(fn ConstructionScript
  (|CallParentFunction))

(fn Init
  (|CallParentFunction)
  (Default|Init (Variables|Default|GetBPC_Shield_And_Health) 1e+02 1e+02 0.0 0.0 0.0 "30.000000,30.000000,30.000000" true false))

(fn SpawnMiniMapIcon
  (Game|SpawnActorfromClass "/Game/Star-Map/Blueprints/UX/BP_MiniMapIcon.BP_MiniMapIcon_C" (Math|Transform|MakeTransform (Transformation|GetWorldLocation (Variables|Default|GetDefaultSceneRoot)) "0, 0, 0" "10.000000,10.000000,10.000000") "Undefined" 0 "/Game/Star-Map/Assets/Sprites/Icons/Objective_Sprite.Objective_Sprite" 0))