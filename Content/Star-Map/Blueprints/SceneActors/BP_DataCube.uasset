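; Data cube scene actor that stays shielded until all of its linked power supply units are destroyed, then becomes triggerable.
; Init sets up the shield/health component, spawns a beam particle system per supply and binds to each supply's destruction.
; Each destruction decrements the count, drops the shield at zero and re-aims beams from cube to remaining supplies.
; Hits while shielded pass zero damage to the health component.
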(event Custom|OnBindToSupplyUnits
  (if (> (Utilities|Array|Length (Variables|Shield|GetPowerSupplies)) 0)
    (for _array_element (Variables|Shield|GetPowerSupplies)
      (Game|BindEventtoOnDestroyed _array_element (delegate Custom|OnSupplyUnitDestroyed))
      (CallFunction|UpdateBeamVFX))))

(event Custom|OnSupplyUnitDestroyed
  (params (DestroyedActor :type Actor%20Object%20Reference))
  (Game|UnbindEventfromOnDestroyed DestroyedActor (delegate Custom|OnSupplyUnitDestroyed))
  (Math|Integer|DecrementInt (Variables|Shield|GetPowerSupplyUnitsLeft)
    (:%20%20
      (CallFunction|EvaluateCanbeTriggered)
      (CallFunction|UpdateBeamVFX))))

(event EventBeginPlay
  (CallFunction|Init))

(event Collision|EventActorBeginOverlap
  (params (OtherActor :type Actor%20Object%20Reference))
  (|CallParentFunction OtherActor) ; This node is disabled and will not be called.\nDrag off pins to build functionality.
)

(event EventTick
  (params (DeltaSeconds :type Float%20%28single-precision%29))
  (|CallParentFunction DeltaSeconds) ; This node is disabled and will not be called.\nDrag off pins to build functionality.
)

(event EventApplyDamage
  (params (Damage :type Float%20%28single-precision%29) (Instigator :type Actor%20Object%20Reference))
  ;[1 1 1] On damaged on be damaged when it can't be triggered
  (if (not (Variables|Default|GetCanBeTriggered))
    (Default|OnDamageTaken (Variables|Default|GetBPC_Shield_And_Health) 0.0)))

(fn ConstructionScript
  (|CallParentFunction))

(fn Init
  (|CallParentFunction)
  (Default|Init (Variables|Default|GetBPC_Shield_And_Health) 1e+02 1e+02 0.0 0.0 0.0 "50.000000,50.000000,50.000000" true false)
  (CallFunction|SetUpBeamEffect)
  (CallFunction|SetUpShieldSupplies))

(fn SetUpShieldSupplies
  (Variables|Shield|SetPowerSupplyUnitsLeft (Utilities|Array|Length (Variables|Shield|GetPowerSupplies)))
  (CallFunction|OnBindtoSupplyUnits))

(fn EvaluateCanbeTriggered
  (if (<= (Variables|Shield|GetPowerSupplyUnitsLeft) 0)
    (Variables|Default|SetCanBeTriggered true)
    (Default|RemoveShield (Variables|Default|GetBPC_Shield_And_Health))))

(fn SetUpBeamEffect
  (for _index (range 0 (- (Utilities|Array|Length (Variables|Shield|GetPowerSupplies)) 1))
    (bind _returnvalue (AddComponent|AddParticleSystemComponent false))
    (Utilities|Array|Add (Variables|VFX|GetParticleSystems) _returnvalue)))

(fn UpdateBeamVFX
  ;[1 1 1] Get null elements
  (for (_array_element _array_index) (Variables|Shield|GetPowerSupplies)
    (Utilities|IsValid _array_element
      (:Is%20Not%20Valid
        (Utilities|Array|Add (LocalVariables|GetelementsToClear) _array_index))))
  ;[1 1 1] Remove Elements
  (for _array_element_2 (LocalVariables|GetelementsToClear)
    (Utilities|Array|RemoveIndex (Variables|Shield|GetPowerSupplies) _array_element_2))
  ;[1 1 1] Clear Emitters no in use
  (CallFunction|ClearUnusedEmiters)
  ;[1 1 1] Update All remaining emitters
  (for (_array_element_3 _array_index_2) (Variables|Shield|GetPowerSupplies)
    (Utilities|IsValid (Utilities|Array|Get(acopy) (Variables|VFX|GetParticleSystems) _array_index_2)
      (:Is%20Valid
        (Class|ParticleSystemComponent|SetBeamSourcePoint (Utilities|Array|Get(acopy) (Variables|VFX|GetParticleSystems) _array_index_2) 0 (Transformation|GetActorLocation))
        (Class|ParticleSystemComponent|SetBeamTargetPoint (Utilities|Array|Get(acopy) (Variables|VFX|GetParticleSystems) _array_index_2) 0 (Transformation|GetActorLocation _array_element_3))))))

(fn ClearUnusedEmiters
  (bind _returnvalue (Transformation|GetActorLocation))
  (bind _powersupplies (Variables|Shield|GetPowerSupplies))
  (bind _particlesystems (Variables|VFX|GetParticleSystems))
  (bind _returnvalue_2 (* _returnvalue 1e+07))
  ;[1 1 1] If the number of p systems is greater than n supplies trim
  (if (> (Utilities|Array|Length _powersupplies) (Utilities|Array|Length _particlesystems))
    (for _index (range (Utilities|Array|LastIndex _powersupplies) (Utilities|Array|LastIndex _particlesystems))
      ;[1 1 1] Remove and destroy component
      (Utilities|IsValid (Utilities|Array|Get(acopy) (Variables|VFX|GetParticleSystems) _index)
        (:Is%20Valid
          (Utilities|Array|RemoveItem (Variables|VFX|GetParticleSystems) (Utilities|Array|Get(acopy) (Variables|VFX|GetParticleSystems) _index))
          (Class|ParticleSystemComponent|SetBeamTargetPoint (Utilities|Array|Get(acopy) (Variables|VFX|GetParticleSystems) _index) 0 _returnvalue_2)
          (Class|ParticleSystemComponent|SetBeamSourcePoint (Utilities|Array|Get(acopy) (Variables|VFX|GetParticleSystems) _index) 0 _returnvalue_2)
          (Components|DestroyComponent (Utilities|Array|Get(acopy) (Variables|VFX|GetParticleSystems) _index)))))))