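; Base actor for star-map objectives, with an empty ObjectiveComplete function as a placeholder for completion logic.
; Shortly after BeginPlay, Init gives RotatingMovement a random spin within MaxRotation and initializes the points-of-interest component.
; SpawnMiniMapIcon can place an objective-sprite icon at the actor's location, but nothing here calls it.
; Team queries use one hardcoded team, though GetTeam reports it as invalid while IsOnTeam reports valid.
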(event EventBeginPlay
  (Utilities|FlowControl|Delay 0.2)
  (CallFunction|Init))

(event Collision|EventActorBeginOverlap
  (params (OtherActor :type Actor%20Object%20Reference)))

(event EventTick
  (params (DeltaSeconds :type Float%20%28single-precision%29)))

(fn ConstructionScript)

(fn ObjectiveComplete)

(fn Init
  (CallFunction|SetRandomRotation)
  (Default|OnInit (Variables|Default|GetBPC_PointsOfInterest)))

(fn SetRandomRotation
  (bind _maxrotation (Variables|VFX|GetMaxRotation))
  (Variables|/Script/Engine.RotatingMovementComponent|SetRotationRate (Variables|Default|GetRotatingMovement) (Math|Rotator|MakeRotator (Math|Random|RandomFloatinRange (* -1 (.x _maxrotation)) (.x _maxrotation)) (Math|Random|RandomFloatinRange (* -1 (.y _maxrotation)) (.y _maxrotation)) (Math|Random|RandomFloatinRange (* -1 (.z _maxrotation)) (.z _maxrotation)))))

(fn SpawnMiniMapIcon
  (Game|SpawnActorfromClass "/Game/Star-Map/Blueprints/UX/BP_MiniMapIcon.BP_MiniMapIcon_C" (Math|Transform|MakeTransform (Transformation|GetActorLocation) "0, 0, 0" "30.000000,30.000000,30.000000") "Undefined" 0 "/Game/Star-Map/Assets/Sprites/Icons/Objective_Sprite.Objective_Sprite" 0))

(fn GetTeam
  (return false "NewEnumerator1"))

(fn IsonTeam
  (params (OtherTeam :type E_Teams%20Enum :default "NewEnumerator0"))
  (return (Utilities|Enum|Equal(Enum) OtherTeam "NewEnumerator1") true))