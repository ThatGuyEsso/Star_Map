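; PC_LoadOut is a player controller, named for a loadout mode, that relays directional input to its pawn.
; Right, Up, Left and Down input actions each send separate press and release messages to the controlled pawn.
; The controller holds no other logic, leaving the response to each direction entirely to the pawn.
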(event Input|ActionEvents|InputActionRight
  (params (Key :type Key%20Structure :default "None"))
  (bind _returnvalue (Pawn|GetControlledPawn))
  (:Pressed
    (Class|I2DMovement|OnRightDown(Message) _returnvalue))
  (:Released
    (Class|I2DMovement|OnRightRelease(Message) _returnvalue)))

(event Input|ActionEvents|InputActionLeft
  (params (Key :type Key%20Structure :default "None"))
  (bind _returnvalue (Pawn|GetControlledPawn))
  (:Pressed
    (Class|I2DMovement|OnLeftDown(Message) _returnvalue))
  (:Released
    (Class|I2DMovement|OnLeftRelease(Message) _returnvalue)))

(event Input|ActionEvents|InputActionUp
  (params (Key :type Key%20Structure :default "None"))
  (bind _returnvalue (Pawn|GetControlledPawn))
  (:Pressed
    (Class|I2DMovement|OnUpDown(Message) _returnvalue))
  (:Released
    (Class|I2DMovement|OnUpRelease(Message) _returnvalue)))

(event Input|ActionEvents|InputActionDown
  (params (Key :type Key%20Structure :default "None"))
  (bind _returnvalue (Pawn|GetControlledPawn))
  (:Pressed
    (Class|I2DMovement|OnDownDown(Message) _returnvalue))
  (:Released
    (Class|I2DMovement|OnDownRelease(Message) _returnvalue)))

(fn ConstructionScript)