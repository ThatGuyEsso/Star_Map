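; Player controller for the player's ship, translating input into message calls on the controlled pawn for strafing, thrust, braking, primary fire and weapon toggles, and on the game mode for pause.
; Each weapon toggle key reads the type shown in its HUD slot, toggles that type on the pawn and updates the slot.
; HUD setup creates the W_HUD widget, seeds it with hull and shield health, requests weapon display and adds the minimap.
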(event EventBeginPlay
  (Variables|Default|SetbShowMouseCursor true))

(event EventSetUpHUD
  (CallFunction|SetUpPlayerHUD))

(event Input|ActionEvents|InputActionStopShip
  (params (Key :type Key%20Structure :default "None"))
  (bind _returnvalue (Pawn|GetControlledPawn))
  (:Pressed
    (Class|ISpaceShip|OnBrake(Message) _returnvalue))
  (:Released
    (Class|ISpaceShip|OnStopBraking(Message) _returnvalue)))

(event Input|ActionEvents|InputActionPrimaryFIre
  (params (Key :type Key%20Structure :default "None"))
  (bind _returnvalue (Pawn|GetControlledPawn))
  (:Pressed
    (Class|ISpaceShip|OnFirePrimary(Message) _returnvalue))
  (:Released
    (Class|ISpaceShip|OnStopFiringPrimary(Message) _returnvalue)))

(event Input|ActionEvents|InputActionToggleWeapon0
  (params (Key :type Key%20Structure :default "None"))
  (bind _hud (Variables|Default|GetHUD))
  ;[1 1 1] Toggle weapons used
  (:Pressed
    (bind _type (Default|GetDispayedType _hud))
    (Class|ISpaceShip|OnToggleWeaponsOfType(Message) (Pawn|GetControlledPawn) _type)
    (Class|IHUD|OnToggleElement(Message) _hud)))

(event Input|ActionEvents|InputActionToggleWeapon1
  (params (Key :type Key%20Structure :default "None"))
  (bind _hud (Variables|Default|GetHUD))
  ;[1 1 1] Toggle weapons used
  (:Pressed
    (bind _type (Default|GetDispayedType _hud 1))
    (Class|ISpaceShip|OnToggleWeaponsOfType(Message) (Pawn|GetControlledPawn) _type)
    (Class|IHUD|OnToggleElement(Message) _hud 1)))

(event Input|ActionEvents|InputActionToggleWeapon3
  (params (Key :type Key%20Structure :default "None"))
  (bind _hud (Variables|Default|GetHUD))
  ;[1 1 1] Toggle weapons used
  (:Pressed
    (bind _type (Default|GetDispayedType _hud 3))
    (Class|ISpaceShip|OnToggleWeaponsOfType(Message) (Pawn|GetControlledPawn) _type)
    (Class|IHUD|OnToggleElement(Message) _hud 3)))

(event Input|ActionEvents|InputActionThrust
  (params (Key :type Key%20Structure :default "None"))
  (bind _returnvalue (Pawn|GetControlledPawn))
  (:Pressed
    (Class|ISpaceShip|OnApplyThrust(Message) _returnvalue))
  (:Released
    (Class|ISpaceShip|OnStopThrusting(Message) _returnvalue)))

(event Input|ActionEvents|InputActionToggleWeapon2
  (params (Key :type Key%20Structure :default "None"))
  (bind _hud (Variables|Default|GetHUD))
  ;[1 1 1] Toggle weapons used
  (:Pressed
    (bind _type (Default|GetDispayedType _hud 2))
    (Class|ISpaceShip|OnToggleWeaponsOfType(Message) (Pawn|GetControlledPawn) _type)
    (Class|IHUD|OnToggleElement(Message) _hud 2)))

(event Input|ActionEvents|InputActionTogglePause
  (params (Key :type Key%20Structure :default "None"))
  (:Pressed
    (Class|IStarMap|OnTogglePause(Message) (Game|GetGameMode))))

(event Input|AxisEvents|InputAxisMoveRight
  (params (AxisValue :type Float%20%28single-precision%29))
  (Class|ISpaceShip|ApplyStrafe(Message) (Pawn|GetControlledPawn) AxisValue))

(fn ConstructionScript)

(fn SetUpPlayerHUD
  (bind _returnvalue (UserInterface|CreateWidget "/Game/Star-Map/Blueprints/Widget/W_HUD.W_HUD_C"))
  (bind _output_get (Variables|Default|SetHUD _returnvalue))
  (UserInterface|Viewport|AddtoViewport _output_get 0)
  (bind _percentshieldhealth (Class|IPlayerShip|GetCurrentPercentageShieldHealth(Message) (Pawn|GetControlledPawn)))
  (bind _percenthealth (Class|IPlayerShip|GetCurrentPercentageHealth(Message) (Pawn|GetControlledPawn)))
  (Default|Init (Variables|Default|GetHUD) _percentshieldhealth _percenthealth)
  (Class|ISpaceShip|OnDisplayWeapons(Message) (Pawn|GetControlledPawn))
  (Default|AddMinimapImage (Variables|Default|GetHUD)))

(fn GetPlayerHUD
  (return (Variables|Default|GetHUD)))