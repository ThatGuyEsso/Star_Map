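; Base gun weapon that fires projectiles from its fire point when enabled, off cooldown and supplied with ammo.
; Each shot spawns a BP_BaseProjectile, decrements ammo and starts a timer that re-enables firing; zero max ammo means unlimited shots.
; For one team only, firing updates the player HUD's ammo and runs a fast looping timer that refreshes the cooldown display until the gun is ready.
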(event Custom|OnUpdateTImer
  (if (Variables|GunSettings|GetcanFire)
    (Utilities|Time|PauseTimerbyHandle (Variables|Default|GetUpdateTimer))
    (CallFunction|HideCoolDownDisplay)
    (else
      (CallFunction|UpdateCooldown))))

(event EventInitWeapon
  (params (Team :type E_Teams%20Enum :default "NewEnumerator0"))
  (CallFunction|Init Team))

(event EventUpdateHUDDisplay
  (CallFunction|UpdateAmmoDisplay))

(event EventSetIsEnabled
  (params (isEnabled :type Boolean))
  (Variables|GunSettings|SetIsGunEnabled isEnabled))

(event EventUseWeapon
  (params (Owner :type Actor%20Object%20Reference))
  (bind _returnvalue (CallFunction|HasAmmo))
  (if (Math|Boolean|ANDBoolean (Variables|GunSettings|GetIsGunEnabled) (Variables|GunSettings|GetcanFire) _returnvalue)
    (CallFunction|Fire Owner)
    (if (Utilities|Enum|Equal(Enum) (Variables|Default|GetTeam) "NewEnumerator0")
      (CallFunction|UpdateAmmoDisplay)
      (CallFunction|ShowCooldownDisplay)
      (bind _returnvalue_2 (Utilities|Time|SetTimerbyEvent (delegate Custom|OnUpdateTImer) 0.01 true))
      (Variables|Default|SetUpdateTimer _returnvalue_2))))

(fn ConstructionScript)

(fn Fire
  (params (Owner :type Actor%20Object%20Reference))
  (bind _firepoint (Variables|Default|GetFirePoint))
  (Variables|GunSettings|SetcanFire false)
  (Game|SpawnActorfromClass "/Game/Star-Map/Blueprints/Projectiles/BP_BaseProjectile.BP_BaseProjectile_C" (Math|Transform|MakeTransform (Transformation|GetWorldLocation _firepoint) (Transformation|GetWorldRotation _firepoint) "1,1,1") "Undefined" Owner (Variables|GunSettings|GetProjectileLifeTime) (Variables|GunSettings|GetProjectileSpeed) (Math|Vector|GetForwardVector (Variables|Default|GetFirePoint)) 5.0 0)
  (bind _returnvalue (Utilities|Time|SetTimerbyFunctionName 0 "ResetCanFire" (Variables|GunSettings|GetTimeBetweenShots)))
  (Variables|Default|SetcooldownTimer _returnvalue)
  (Math|Integer|DecrementInt (Variables|GunSettings|GetcurrentAmmo)))

(fn ResetCanFire
  (Variables|GunSettings|SetcanFire true))

(fn Init
  (params (Team :type E_Teams%20Enum :default "NewEnumerator0"))
  (Variables|GunSettings|SetcurrentAmmo (Variables|GunSettings|GetmaxAmmo))
  (Variables|Default|SetTeam Team))

(fn UpdateAmmoDisplay
  (bind _hud (Class|IPlayerController|GetPlayerHUD(Message) (Game|GetPlayerController 0)))
  (Utilities|IsValid _hud
    (:Is%20Valid
      (Default|UpdateAmmoDisplay _hud (Variables|Default|GetweaponType) (Variables|GunSettings|GetcurrentAmmo)))))

(fn HasAmmo
  (return (or (> (Variables|GunSettings|GetcurrentAmmo) 0) (== (Variables|GunSettings|GetmaxAmmo) 0))))

(fn UpdateCooldown
  (bind _hud (Class|IPlayerController|GetPlayerHUD(Message) (Game|GetPlayerController 0)))
  (Utilities|IsValid _hud
    (:Is%20Valid
      (Default|UpdateCooldownDisplay _hud (Variables|Default|GetweaponType) (Math|Integer|Clamp(Integer) (Math|Float|Floor (- (Variables|GunSettings|GetTimeBetweenShots) (Class|KismetSystemLibrary|GetTimerElapsedTimeHandle (Variables|Default|GetcooldownTimer)))) 0 (Math|Float|Ceil (Variables|GunSettings|GetTimeBetweenShots)))))))

(fn ShowCooldownDisplay
  (bind _hud (Class|IPlayerController|GetPlayerHUD(Message) (Game|GetPlayerController 0)))
  (Utilities|IsValid _hud
    (:Is%20Valid
      (Class|IHUD|ShowCooldown(Message) _hud (Variables|Default|GetweaponType) (Math|Float|Truncate (Variables|GunSettings|GetTimeBetweenShots))))))

(fn HideCoolDownDisplay
  (bind _hud (Class|IPlayerController|GetPlayerHUD(Message) (Game|GetPlayerController 0)))
  (Utilities|IsValid _hud
    (:Is%20Valid
      (Class|IHUD|RemoveCoolDown(Message) _hud (Variables|Default|GetweaponType)))))

(fn GetWeaponType
  (return (Variables|Default|GetweaponType)))

(fn IsEnabled
  (return (Variables|GunSettings|GetIsGunEnabled)))