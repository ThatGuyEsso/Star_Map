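; Missile launcher weapon Blueprint whose Fire function spawns a BP_Missile at the FirePoint component, aimed along its forward vector.
; The missile receives the passed-in owner plus speed, damage and lifetime from GunSettings.
; Each shot clears CanFire, starts a stored cooldown timer that calls ResetCanFire by name, and decrements CurrentAmmo.
; Fire itself checks neither ammo nor cooldown, and the event graph holds no active logic.
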(event EventBeginPlay)

(event Collision|EventActorBeginOverlap
  (params (OtherActor :type Actor%20Object%20Reference)))

(event EventTick
  (params (DeltaSeconds :type Float%20%28single-precision%29)))

(fn ConstructionScript
  (|CallParentFunction))

(fn Fire
  (params (Owner :type Actor%20Object%20Reference))
  (bind _firepoint (Variables|Default|GetFirePoint))
  (bind _gunsettings (Variables|Default|GetGunSettings))
  (Variables|Default|SetcanFire false)
  (Game|SpawnActorfromClass "/Game/Star-Map/Blueprints/Projectiles/BP_Missile.BP_Missile_C" (Math|Transform|MakeTransform (Transformation|GetWorldLocation _firepoint) (Transformation|GetWorldRotation _firepoint) "1,1,1") "Undefined" Owner (.projectilelifetime _gunsettings) (.projectilespeed _gunsettings) (Math|Vector|GetForwardVector (Variables|Default|GetFirePoint)) (.damage _gunsettings) 0)
  (bind _returnvalue (Utilities|Time|SetTimerbyFunctionName 0 "ResetCanFire" (.timebetweenshots _gunsettings)))
  (Variables|Default|SetcooldownTimer _returnvalue)
  (Math|Integer|DecrementInt (Variables|Default|GetcurrentAmmo)))