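; Ship-mounted laser weapon that fires a sustained beam while its owning ship attacks, bound through BP_BaseShip attack events.
; Tick line-traces every frame to place the beam particle endpoints, applying damage only at the fire-rate interval.
; Releasing attack or exhausting beam duration starts a long cooldown, with a looping timer updating the player's HUD.
; Helpers manage attached fire and looping beam audio, plus explosion VFX with team-conditional camera shake.
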(event Custom|OnBindToShipAttack
  (bind _asbp_base_ship (Utilities|Casting|CastToBP_BaseShip (Variables|Default|GetowningShip)))
  (EventDispatchers|BindEventtoOnTryingtoAttack _asbp_base_ship (delegate Custom|OnAttack))
  (EventDispatchers|BindEventtoOnStopTryingtoAttack _asbp_base_ship (delegate Custom|OnStopAttack)))

(event Custom|OnAttack
  (if (Variables|Default|GetIsGunEnabled)
    (Variables|GunSettings|SetOnIsAttacking true)
    (if (Variables|GunSettings|GetIsOnCoolDown)
      _)))

(event Custom|OnStopAttack
  (if (Variables|GunSettings|GetOnIsAttacking)
    (Variables|GunSettings|SetOnIsAttacking false)
    (if (Actor|ActorHasTag (Variables|Default|GetowningShip) "Player")
      (CallFunction|UpdateAmmoDisplay)
      (CallFunction|ShowCooldownDisplay))
    (CallFunction|OnBeginBeamCooldown)))

(event Custom|OnBeginBeamCooldown
  (if (not (Variables|GunSettings|GetIsOnCoolDown))
    (Variables|GunSettings|SetIsOnCoolDown true)
    (CallFunction|StopDrawing)
    (CallFunction|StopBeamSFX)
    (bind _returnvalue (Utilities|Time|SetTimerbyEvent (delegate EventOnUpdateTImer) 0.01 true))
    (Variables|Default|SetUpdateTimer _returnvalue)
    (bind _returnvalue_2 (Utilities|Time|SetTimerbyFunctionName 0 "ResetLongCooldown" (Variables|GunSettings|GetLongCoolDownTime)))
    (Variables|GunSettings|SetLongCooldownTimer _returnvalue_2)))

(event EventSetIsAttacking
  (params (IsAttacking :type Boolean))
  (if IsAttacking
    (CallFunction|OnAttack)
    (else
      (CallFunction|OnStopAttack))))

(event Collision|EventActorBeginOverlap
  (params (OtherActor :type Actor%20Object%20Reference)))

(event EventTick
  (params (DeltaSeconds :type Float%20%28single-precision%29))
  (bind _beamaudioplayer (Variables|Default|GetBeamAudioPlayer))
  (if (Math|Boolean|ANDBoolean (Variables|Default|GetIsGunEnabled) (Variables|GunSettings|GetOnIsAttacking) (not (Variables|GunSettings|GetIsOnCoolDown)))
    (Utilities|IsValid _beamaudioplayer
      (:Is%20Valid
        _)
      (:Is%20Not%20Valid
        (CallFunction|SetUpBeamDurationSFX)))
    (bind _isplaying (Default|IsPlaying _beamaudioplayer))
    (if _isplaying
      _
      (else
        (CallFunction|PlayFireSFX)
        (CallFunction|PlayBeamSFX)))
    (CallFunction|SpawnExplosionat (Variables|Default|GetMuzzleExplosion) (Transformation|GetWorldLocation (Variables|Default|GetFirePoint)))
    (if (Variables|Default|GetcanFire)
      (CallFunction|Fire (Variables|Default|GetowningShip))
      (CallFunction|DrawBeamVFX)
      (else
        (CallFunction|DoRangeCast)
        (CallFunction|DrawBeamVFX)))
    (bind _output_get (Variables|GunSettings|SetcurrentBeamDureation (- (Variables|GunSettings|GetcurrentBeamDureation) DeltaSeconds)))
    (if (<= _output_get 0.0)
      (CallFunction|OnBeginBeamCooldown))))

(event EventUseWeapon
  (params (Owner :type Actor%20Object%20Reference))
  ;[1 1 1] Just need to override it
)

(event EventOnUpdateTImer
  (if (Variables|GunSettings|GetIsOnCoolDown)
    (CallFunction|UpdateCooldown)
    (else
      (Utilities|Time|PauseTimerbyHandle (Variables|Default|GetUpdateTimer))
      (if (Actor|ActorHasTag (Variables|Default|GetowningShip) "Player")
        (CallFunction|HideCoolDownDisplay)))))

(fn ConstructionScript
  (|CallParentFunction))

(fn Fire
  (params (Owner :type Actor%20Object%20Reference))
  (Variables|Default|SetcanFire false)
  (CallFunction|DoDamageCast)
  (Utilities|Time|SetTimerbyFunctionName 0 "ResetCanFire" (.timebetweenshots (Variables|Default|GetGunSettings))))

(fn DoDamageCast
  (bind _firepoint (Variables|Default|GetFirePoint))
  (bind _owningship (Variables|Default|GetowningShip))
  (bind _firepoint_2 (Variables|Default|GetFirePoint))
  (bind _returnvalue (Transformation|GetWorldLocation _firepoint_2))
  (bind (_outhit _returnvalue_2) (Collision|LineTraceByChannel _returnvalue (+ _returnvalue (* (Math|Vector|GetForwardVector _firepoint_2) (Variables|GunSettings|GetRange))) "TraceTypeQuery1" false 0 "None"))
  (if _returnvalue_2
    (Variables|VFX|SetcurrentTargetPoint (.ImpactPoint (Collision|BreakHitResult _outhit)))
    (if (!= (Components|GetOwner (Variables|/Script/Engine.Actor|GetRootComponent (.HitActor (Collision|BreakHitResult _outhit)))) self)
      (if (!= (Components|GetOwner (Variables|/Script/Engine.Actor|GetRootComponent (.HitActor (Collision|BreakHitResult _outhit)))) _owningship)
        (Class|IDamage|ApplyDamage(Message) (Components|GetOwner (Variables|/Script/Engine.Actor|GetRootComponent (.HitActor (Collision|BreakHitResult _outhit)))) (.damage (Variables|Default|GetGunSettings)) _owningship)
        (CallFunction|SpawnExplosionat (Variables|VFX|GetHitVFXSettings) (Variables|VFX|GetcurrentTargetPoint))))
    (else
      (Variables|VFX|SetcurrentTargetPoint (+ (Transformation|GetWorldLocation _firepoint) (* (Math|Vector|GetForwardVector _firepoint) (Variables|GunSettings|GetRange)))))))

(fn DrawBeamVFX
  (bind _beam (Variables|Default|GetBeam))
  (if (Components|Activation|IsActive (Variables|Default|GetBeam))
    _
    (else
      (Components|Activation|Activate _beam true)))
  (Class|ParticleSystemComponent|SetBeamSourcePoint _beam 0 (Transformation|GetWorldLocation (Variables|Default|GetFirePoint)))
  (Class|ParticleSystemComponent|SetBeamTargetPoint _beam 0 (Variables|VFX|GetcurrentTargetPoint))
  (CallFunction|SpawnExplosionat :spawnPoint (Variables|VFX|GetcurrentTargetPoint)))

(fn Init
  (params (Team :type E_Teams%20Enum :default "NewEnumerator0") (owningShip :type Actor%20Object%20Reference))
  (|CallParentFunction Team owningShip)
  (Components|Activation|Deactivate (Variables|Default|GetBeam))
  (CallFunction|OnBindtoShipAttack)
  (Variables|GunSettings|SetcurrentBeamDureation (Variables|GunSettings|GetMaxBeamDuration)))

(fn DoRangeCast
  (bind _firepoint (Variables|Default|GetFirePoint))
  (bind _firepoint_2 (Variables|Default|GetFirePoint))
  (bind _returnvalue (Transformation|GetWorldLocation _firepoint_2))
  (bind (_outhit _returnvalue_2) (Collision|LineTraceByChannel _returnvalue (+ _returnvalue (* (Math|Vector|GetForwardVector _firepoint_2) (Variables|GunSettings|GetRange))) "TraceTypeQuery1" false 0 "None"))
  (if _returnvalue_2
    (Variables|VFX|SetcurrentTargetPoint (.ImpactPoint (Collision|BreakHitResult _outhit)))
    (if (!= (Components|GetOwner (Variables|/Script/Engine.Actor|GetRootComponent (.HitActor (Collision|BreakHitResult _outhit)))) self)
      (if (!= (Components|GetOwner (Variables|/Script/Engine.Actor|GetRootComponent (.HitActor (Collision|BreakHitResult _outhit)))) (Components|GetOwner))
        _))
    (else
      (Variables|VFX|SetcurrentTargetPoint (+ (Transformation|GetWorldLocation _firepoint) (* (Math|Vector|GetForwardVector _firepoint) (Variables|GunSettings|GetRange)))))))

(fn StopDrawing
  (bind _beam (Variables|Default|GetBeam))
  (bind _owningship (Variables|Default|GetowningShip))
  (bind _returnvalue (Transformation|GetActorLocation _owningship))
  (bind _returnvalue_2 (* _returnvalue 1e+07))
  (if (Components|Activation|IsActive (Variables|Default|GetBeam))
    (Class|ParticleSystemComponent|SetBeamTargetPoint _beam 0 _returnvalue_2)
    (Class|ParticleSystemComponent|SetBeamSourcePoint _beam 0 _returnvalue_2)
    (Components|Activation|Deactivate _beam)))

(fn UpdateCooldown
  (if (Actor|ActorHasTag (Variables|Default|GetowningShip) "Player")
    (bind _hud (Class|IPlayerController|GetPlayerHUD(Message) (Game|GetPlayerController 0)))
    (Utilities|IsValid _hud
      (:Is%20Valid
        (Default|UpdateCooldownDisplay _hud (Variables|Default|GetweaponType) (Math|Integer|Clamp(Integer) (Math|Float|Floor (- (Variables|GunSettings|GetLongCoolDownTime) (Class|KismetSystemLibrary|GetTimerElapsedTimeHandle (Variables|GunSettings|GetLongCooldownTimer)))) 0 (Math|Float|Ceil (Variables|GunSettings|GetLongCoolDownTime))))))))

(fn ResetLongCooldown
  (Variables|GunSettings|SetIsOnCoolDown false)
  (Variables|GunSettings|SetcurrentBeamDureation (Variables|GunSettings|GetMaxBeamDuration)))

(fn ResetCanFire
  (|CallParentFunction))

(fn PlayFireSFX
  (bind _self self)
  (bind _returnvalue (Game|SpawnActorfromClass "/Game/Star-Map/Blueprints/UX/BP_AudioPlayer.BP_AudioPlayer_C" (Math|Transform|MakeTransform (Transformation|GetActorLocation) "0, 0, 0" "1,1,1") "Undefined" 0 (Variables|Default|GetFireSFX) true false false 3.0 0))
  (Utilities|IsValid _self
    (:Is%20Valid
      (Utilities|IsValid _returnvalue
        (:Is%20Valid
          (Transformation|AttachActorToActor _returnvalue _self "None" "KeepRelative" "KeepRelative" "KeepRelative" false))))))

(fn SetUpBeamDurationSFX
  (bind _self self)
  (bind _returnvalue (Game|SpawnActorfromClass "/Game/Star-Map/Blueprints/UX/BP_AudioPlayer.BP_AudioPlayer_C" (Math|Transform|MakeTransform (Transformation|GetActorLocation) "0, 0, 0" "1,1,1") "Undefined" 0 (Variables|Default|GetBeamMaintainSFX) false true false 3.0 0))
  (Variables|Default|SetBeamAudioPlayer _returnvalue)
  (Utilities|IsValid _self
    (:Is%20Valid
      (Utilities|IsValid _returnvalue
        (:Is%20Valid
          (Transformation|AttachActorToActor _returnvalue _self "None" "KeepRelative" "KeepRelative" "KeepRelative" false)
          (Default|StopSound _returnvalue))))))

(fn PlayBeamSFX
  (bind _beamaudioplayer (Variables|Default|GetBeamAudioPlayer))
  (Utilities|IsValid _beamaudioplayer
    (:Is%20Valid
      _)
    (:Is%20Not%20Valid
      (CallFunction|SetUpBeamDurationSFX)))
  (Default|PlaySound _beamaudioplayer))

(fn StopBeamSFX
  (bind _beamaudioplayer (Variables|Default|GetBeamAudioPlayer))
  (Utilities|IsValid _beamaudioplayer
    (:Is%20Valid
      (Default|FadeOut _beamaudioplayer))))

(fn SpawnExplosionat
  (params (VFX%20Settings :type S%20Explosion%20VFX%20Settings%20Structure) (spawnPoint :type Vector :default "0, 0, 0"))
  (Game|SpawnActorfromClass "/Game/Star-Map/Blueprints/VFX/BP_ExplosionManager.BP_ExplosionManager_C" (Math|Transform|MakeTransform spawnPoint "0, 0, 0" "1,1,1") "Undefined" 0 VFX%20Settings false 0)
  (bind (_isvalid _team) (Class|ITeams|GetTeam(Message) (Variables|Default|GetowningShip)))
  (if (and _isvalid (Utilities|Enum|Equal(Enum) _team "NewEnumerator0"))
    (Camera|PlayWorldCameraShake "/Game/Star-Map/Blueprints/UX/CAM_Effects/BP_BeamSustain.BP_BeamSustain_C" (Transformation|GetActorLocation) 0.0 7e+04 1.0 true)))