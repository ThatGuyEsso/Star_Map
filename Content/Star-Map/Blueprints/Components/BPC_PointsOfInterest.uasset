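; Actor component that registers its owner as a point of interest on the player's HUD minimap.
; On init it finds the BP_MinimapCamera and passes its scene capture, with the icon, size, static flag and rotation settings, to the minimap's AddPOI, storing the returned widget.
; It binds to the owner's destruction to remove that icon from the minimap.
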(event Custom|OnDestroy
  (params (DestroyedActor :type Actor%20Object%20Reference))
  (Utilities|IsValid (Variables|Default|GetWidget)
    (:Is%20Valid
      (bind _hud (Class|IPlayerController|GetPlayerHUD(Message) (Game|GetPlayerController 0)))
      (Utilities|IsValid (Variables|/Game/Star-Map/Blueprints/Widget/W_HUD.W_HUD_C|GetMiniMap _hud)
        (:Is%20Valid
          (Default|RemoveIcon (Variables|/Game/Star-Map/Blueprints/Widget/W_HUD.W_HUD_C|GetMiniMap _hud) (Variables|Default|GetWidget)))))))

(event Custom|OnInit
  (Game|BindEventtoOnDestroyed (Components|GetOwner) (delegate Custom|OnDestroy))
  (CallFunction|Init))

(fn Init
  (bind _iconsize (Variables|Default|GetIconSIze))
  (Utilities|IsValid (Components|GetOwner)
    (:Is%20Valid
      (bind _hud (Class|IPlayerController|GetPlayerHUD(Message) (Game|GetPlayerController 0)))
      (bind _returnvalue (Actor|GetActorOfClass "/Game/Star-Map/Blueprints/UX/BP_MinimapCamera.BP_MinimapCamera_C"))
      (bind _output_get (Variables|Default|SetminiMapCamera _returnvalue))
      (bind _widget (Default|AddPOI (Variables|/Game/Star-Map/Blueprints/Widget/W_HUD.W_HUD_C|GetMiniMap _hud) (Variables|Default|GetIcon) (Variables|Default|GetIsStatic) (Components|GetOwner) (Variables|/Game/Star-Map/Blueprints/UX/BP_MinimapCamera.BP_MinimapCamera_C|GetSceneCaptureComponent2D _output_get) (Math|Vector2D|MakeVector2D _iconsize _iconsize) (Variables|Default|GetRotation%20Offset) (Variables|Default|GetShould%20Update%20Rotation)))
      (Variables|Default|SetWidget _widget))))