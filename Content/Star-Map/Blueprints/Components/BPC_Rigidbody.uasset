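; Custom rigidbody component that moves its owning ship on the star map through its own force-based physics.
; Each tick it sums queued forces, divides by ship mass for acceleration, moves the owner with a swept location update, then integrates velocity clamped to max speed.
; Braking adds a drag force scaling with speed squared and snaps velocity to zero at low speed.
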(event EventTick
  (params (DeltaSeconds :type Float%20%28single-precision%29))
  (if (Variables|State|GetIsBraking)
    (CallFunction|ApplyScalingBrakingForce (Variables|ShipData|GetBrakeForce)))
  (CallFunction|UpdateNetForce)
  (CallFunction|UpdateAcceleration)
  (CallFunction|MoveShip DeltaSeconds)
  (CallFunction|UpdateVelocity DeltaSeconds)
  (Utilities|Array|Clear (Variables|MovementData|GetForces))
  (Variables|MovementData|SetNetForce "0, 0, 0"))

(fn ApplyForce
  (params (force :type Vector))
  (Utilities|Array|Add (Variables|MovementData|GetForces) force))

(fn Init
  (params (ShipMass :type Float%20%28single-precision%29) (BrakeRate :type Float%20%28single-precision%29) (MaxSpeed :type Float%20%28single-precision%29))
  (Variables|ShipData|SetShipMass ShipMass)
  (Variables|ShipData|SetBrakeForce BrakeRate)
  (Variables|ShipData|SetMaxSpeed MaxSpeed))

(fn SetIsBraking
  (params (IsBraking :type Boolean))
  (Variables|State|SetIsBraking IsBraking)
  (Variables|MovementData|SetCurrentAcceleration "0, 0, 0"))

(fn MoveShip
  (params (DeltaTime :type Float%20%28single-precision%29))
  (if (and (< (Math|Vector|VectorLength (Variables|MovementData|GetCurrentVelocity)) 75.0) (Variables|State|GetIsBraking))
    (Variables|MovementData|SetCurrentVelocity "0, 0, 0"))
  (LocalVariables|SettimeStep DeltaTime)
  (bind _output_get (LocalVariables|SetnewPosition (+ (Transformation|GetActorLocation (Components|GetOwner)) (+ (* (Variables|MovementData|GetCurrentVelocity) (LocalVariables|GettimeStep)) (* (Variables|MovementData|GetCurrentAcceleration) (* (LocalVariables|GettimeStep) (LocalVariables|GettimeStep) 0.5))))))
  (Transformation|SetActorLocation (Components|GetOwner) _output_get true false))

(fn UpdateNetForce
  (for _array_element (Variables|MovementData|GetForces)
    (Variables|MovementData|SetNetForce (+ (Variables|MovementData|GetNetForce) _array_element))))

(fn StopShip
  (Variables|MovementData|SetCurrentVelocity "0, 0, 0")
  (Variables|MovementData|SetCurrentAcceleration "0, 0, 0"))

(fn UpdateAcceleration
  (Variables|MovementData|SetCurrentAcceleration (/ (Variables|MovementData|GetNetForce) (Variables|ShipData|GetShipMass))))

(fn UpdateVelocity
  (params (deltaTime :type Float%20%28single-precision%29))
  (if (>= (Math|Vector|VectorLength (+ (Variables|MovementData|GetCurrentVelocity) (* (Variables|MovementData|GetCurrentAcceleration) deltaTime))) (Variables|ShipData|GetMaxSpeed))
    (Variables|MovementData|SetCurrentVelocity (* (Math|Vector|Normalize (+ (Variables|MovementData|GetCurrentVelocity) (* (Variables|MovementData|GetCurrentAcceleration) deltaTime))) (Variables|ShipData|GetMaxSpeed)))
    (else
      (Variables|MovementData|SetCurrentVelocity (+ (Variables|MovementData|GetCurrentVelocity) (* (Variables|MovementData|GetCurrentAcceleration) deltaTime))))))

(fn ApplyScalingBrakingForce
  (params (BreakForce :type Float%20%28single-precision%29))
  (LocalVariables|Setspeed (Math|Vector|VectorLength (Variables|MovementData|GetCurrentVelocity)))
  (LocalVariables|SetvelNorm (Math|Vector|Normalize (Variables|MovementData|GetCurrentVelocity)))
  (LocalVariables|SetdragMag (* (LocalVariables|Getspeed) (LocalVariables|Getspeed) (Variables|Default|GetBrakeConstant) 0.5 BreakForce))
  (bind _output_get (LocalVariables|SetbrakingForce (* (LocalVariables|GetvelNorm) (* (LocalVariables|GetdragMag) -1.0))))
  (Utilities|Array|Add (Variables|MovementData|GetForces) _output_get))

(fn ApplyLinearBreakingForce
  (LocalVariables|SetbrakingForce (* (Math|Vector|Normalize (Variables|MovementData|GetCurrentVelocity)) (* (Variables|ShipData|GetBrakeForce) (Variables|Default|GetBrakeConstant)))))

(fn GetCurrentSpeed
  (return (Math|Vector|VectorLength (Variables|MovementData|GetCurrentVelocity))))