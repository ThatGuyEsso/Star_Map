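; Component that holds shield and hull health, set up through Init, and broadcasts an update when either changes.
; Damage hits the shield first, removing a fixed one point regardless of damage value; hull takes the full value only once the shield is empty.
; Shield hits halt recharge and restart a cooldown timer, longer when depleted, after which Tick refills the shield at a constant rate.
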(event Custom|OnStopRecharge
  (if (Utilities|Time|IsValidTimerHandle (Variables|Default|GetRechargeTimer))
    (Utilities|Time|PauseTimerbyHandle (Variables|Default|GetRechargeTimer)))
  (Variables|Default|SetcanRecharge false)
  (if (<= (Variables|Default|GetCurrentShieldHealth) 0.0)
    (bind _returnvalue (Utilities|Time|SetTimerbyEvent (delegate Custom|OnCanRecharge) (Variables|Default|GetShieldLongCooldown)))
    (Variables|Default|SetRechargeTimer _returnvalue)
    (else
      (bind _returnvalue_2 (Utilities|Time|SetTimerbyEvent (delegate Custom|OnCanRecharge) (Variables|Default|GetShieldShortCoolDown)))
      (Variables|Default|SetRechargeTimer _returnvalue_2))))

(event Custom|OnCanRecharge
  (Variables|Default|SetcanRecharge true))

(event EventTick
  (params (DeltaSeconds :type Float%20%28single-precision%29))
  (if (and (Variables|Default|GetcanRecharge) (< (Variables|Default|GetCurrentShieldHealth) (Variables|Default|GetMaxShieldHealth)))
    (bind _output_get (Variables|Default|SetCurrentShieldHealth (Math|Interpolation|FInterptoConstant (Variables|Default|GetCurrentShieldHealth) (Variables|Default|GetMaxShieldHealth) DeltaSeconds (Variables|Default|GetShieldChargeRate))))
    (Default|CallOnShieldHealthUpdated _output_get)))

(fn Init
  (params (MaxShieldHealth :type Float%20%28single-precision%29) (MaxHullHealth :type Float%20%28single-precision%29) (ShieldChargeRate :type Float%20%28single-precision%29) (ShieldShortCoolDown :type Float%20%28single-precision%29) (ShieldLongCooldown :type Float%20%28single-precision%29))
  (bind _output_get (Variables|Default|SetMaxShieldHealth MaxShieldHealth))
  (Variables|Default|SetCurrentShieldHealth _output_get)
  (bind _output_get_2 (Variables|Default|SetMaxHullHealth MaxHullHealth))
  (Variables|Default|SetCurrentHullHealth _output_get_2)
  (Variables|Default|SetShieldChargeRate ShieldChargeRate)
  (Variables|Default|SetShieldShortCoolDown ShieldShortCoolDown)
  (Variables|Default|SetShieldLongCooldown ShieldLongCooldown))

(fn OnDamageTaken
  (params (damageValue :type Float%20%28single-precision%29))
  (if (> (Variables|Default|GetCurrentShieldHealth) 0.0)
    (bind _output_get (Variables|Default|SetCurrentShieldHealth (Math|Float|Clamp(Float) (- (Variables|Default|GetCurrentShieldHealth) 1.0) 0.0 (Variables|Default|GetMaxShieldHealth))))
    (Default|CallOnShieldHealthUpdated _output_get)
    (CallFunction|OnStopRecharge)
    (else
      (bind _output_get_2 (Variables|Default|SetCurrentHullHealth (Math|Float|Clamp(Float) (- (Variables|Default|GetCurrentHullHealth) damageValue) 0.0 (Variables|Default|GetMaxHullHealth))))
      (Default|CallOnHullHealthUpdated _output_get_2))))

(fn GetShieldData
  (return (Variables|Default|GetCurrentShieldHealth) (Variables|Default|GetMaxShieldHealth)))

(fn GetHullData
  (return (Variables|Default|GetCurrentHullHealth) (Variables|Default|GetMaxHullHealth)))