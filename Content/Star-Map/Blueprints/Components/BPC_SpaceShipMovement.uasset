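; Movement component that moves its owning spaceship in the Star-Map using simple velocity and acceleration integration.
; Force inputs, divided by ship mass, accumulate into acceleration, which is added to velocity each tick without delta-time scaling.
; Each tick teleports the owner by velocity without sweep, then normalizes velocity with MaxSpeed as the tolerance rather than clamping it.
; Braking clears acceleration, ignores new forces and interpolates velocity toward zero at the brake rate.
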(event EventTick
  (params (DeltaSeconds :type Float%20%28single-precision%29))
  (bind _returnvalue (Components|GetOwner))
  (Transformation|SetActorLocation _returnvalue (+ (Transformation|GetActorLocation _returnvalue) (* (Variables|MovementSettings|GetCurrentVelocity) DeltaSeconds)) false true)
  (Variables|MovementSettings|SetCurrentVelocity (+ (Variables|MovementSettings|GetCurrentVelocity) (Variables|MovementSettings|GetCurrentAcceleration)))
  (Variables|MovementSettings|SetCurrentVelocity (Math|Vector|Normalize (Variables|MovementSettings|GetCurrentVelocity) (Variables|ShipData|GetMaxSpeed)))
  (if (Variables|State|GetIsBraking)
    (Variables|MovementSettings|SetCurrentVelocity (Math|Interpolation|VInterpTo (Variables|MovementSettings|GetCurrentVelocity) "0, 0, 0" DeltaSeconds (Variables|ShipData|GetBrakeRate)))))

(fn AccelerateinDirection
  (params (force :type Vector))
  (if (not (Variables|State|GetIsBraking))
    (Variables|MovementSettings|SetCurrentAcceleration (+ (Variables|MovementSettings|GetCurrentAcceleration) (/ force (Variables|ShipData|GetShipMass))))))

(fn Init
  (params (ShipMass :type Float%20%28single-precision%29) (BrakeRate :type Float%20%28single-precision%29))
  (Variables|ShipData|SetShipMass ShipMass)
  (Variables|ShipData|SetBrakeRate BrakeRate))

(fn SetIsBraking
  (params (IsBraking :type Boolean))
  (Variables|State|SetIsBraking IsBraking)
  (Variables|MovementSettings|SetCurrentAcceleration "0, 0, 0"))