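; Ship movement component that drives its owner's physics velocity from movement data supplied through Init.
; Each tick, braking takes priority over acceleration and eases stored velocity toward zero at the deceleration rate.
; Acceleration ramps speed toward max along the forward vector, steering current velocity there at a multiple of the acceleration rate for gradual drift correction.
; Both write linear velocity directly to the owner's main collider.
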(event EventTick
  (params (DeltaSeconds :type Float%20%28single-precision%29))
  (Variables|Default|SetDelta%20Seconds DeltaSeconds)
  (if (Variables|Default|GetIsBraking)
    (CallFunction|BraketoStandStill)
    (elif (Variables|Default|GetIsTryingToAccelerate)
      (CallFunction|Accelerate))))

(fn Init
  (params (S_ShipMovementData :type S%20Ship%20Movement%20Data%20Structure))
  (Variables|Default|SetS_ShipMovementData S_ShipMovementData))

(fn BraketoStandStill
  (bind _output_get (LocalVariables|SetCurrentSpeed (Math|Vector|VectorLength (Variables|Default|GettargetVelocity))))
  (LocalVariables|SetCurrentSpeed (Math|Interpolation|FInterptoConstant _output_get 0.0 (Variables|Default|GetDelta%20Seconds) (.decelleration (Variables|Default|GetS_ShipMovementData))))
  (bind _output_get_2 (Variables|Default|SettargetVelocity (* (Math|Vector|Normalize (Variables|Default|GettargetVelocity)) (LocalVariables|GetCurrentSpeed))))
  (bind _collider (Class|ISpaceShip|GetMainCollider(Message) (Components|GetOwner)))
  (Physics|SetPhysicsLinearVelocity _collider _output_get_2 false "None"))

(fn Accelerate
  (bind _s_shipmovementdata (Variables|Default|GetS_ShipMovementData))
  (bind _output_get (LocalVariables|SetCurrentSpeed (Math|Interpolation|FInterptoConstant (Math|Vector|VectorLength (Transformation|GetVelocity (Components|GetOwner))) (.maxspeed _s_shipmovementdata) (Variables|Default|GetDelta%20Seconds) (.acceleration _s_shipmovementdata))))
  (bind _output_get_2 (Variables|Default|SettargetVelocity (* (Transformation|GetActorForwardVector (Components|GetOwner)) _output_get)))
  (CallFunction|UpdateVelDirection _output_get_2))

(fn UpdateVelDirection
  (params (targetVelocity :type Vector))
  (bind _returnvalue (Components|GetOwner))
  (bind _output_get (Variables|Default|SettargetVelocity (Math|Interpolation|VInterptoConstant (Transformation|GetVelocity _returnvalue) targetVelocity (Variables|Default|GetDelta%20Seconds) (* (.acceleration (Variables|Default|GetS_ShipMovementData)) 3.6))))
  (bind _collider (Class|ISpaceShip|GetMainCollider(Message) _returnvalue))
  (Class|PrimitiveComponent|SetAllPhysicsLinearVelocity _collider _output_get false))