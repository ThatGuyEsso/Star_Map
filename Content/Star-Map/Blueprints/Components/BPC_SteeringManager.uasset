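; BPC_SteeringManager is a steering component that combines steering forces and applies the result to a rigid body.
; Init stores the RigidBody reference, and AddSteeringForce appends each force to the SteeringForces array.
; UpdateSteering applies the sum from CalculateNetforce through the body's ApplyForce.
; Nothing in the component clears the array, and its Tick is unused, so updates depend on external calls.
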(event EventBeginPlay)

(event EventTick
  (params (DeltaSeconds :type Float%20%28single-precision%29)))

(fn Init
  (params (rigidBody :type BPC%20Rigidbody%20Object%20Reference))
  (Variables|Default|SetRigid%20Body rigidBody))

(fn UpdateSteering
  (bind _resultantforce (CallFunction|CalculateNetforce))
  (Default|ApplyForce (Variables|Default|GetRigid%20Body) _resultantforce))

(fn AddSteeringForce
  (params (force :type Vector%20%28by%20ref%29))
  (Utilities|Array|Add (Variables|Default|GetSteeringForces) force))

(fn CalculateNetforce
  (if (> (Utilities|Array|Length (Variables|Default|GetSteeringForces)) 0)
    (for _array_element (Variables|Default|GetSteeringForces)
      (LocalVariables|SetNetForce (+ _array_element (LocalVariables|GetNetForce))))
    (return (LocalVariables|GetNetForce))))